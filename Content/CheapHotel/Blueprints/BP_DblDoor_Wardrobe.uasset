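; Wardrobe actor with double doors that fly open quickly, then creak slowly closed.
; BeginPlay stores both doors' starting rotations, and two timelines drive the yaw, mirrored for the right door, while keeping the original roll and pitch.
; FastOpenDoors plays a sound and the open timeline, which calls SlowCloseDoors on finish to play a creak and the close timeline.
; The close timeline uses Play rather than PlayFromStart, and nothing in this graph calls FastOpenDoors.
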(event `self.ReceiveBeginPlay`
  (set `self.Left Starting Rotation` (`SceneComponent.RelativeRotation` (`self.S_Wardrobe_Door_L`)))
  (set `self.Right Starting Rotation` (`SceneComponent.RelativeRotation` (`self.S_Wardrobe_Door_R`))))

(event `Fast Open Doors`
  (bind (_left_starting_rotation_roll _left_starting_rotation_pitch) (`KismetMathLibrary.BreakRotator` (`self.Left Starting Rotation`)))
  (bind (_right_starting_rotation_roll _right_starting_rotation_pitch) (`KismetMathLibrary.BreakRotator` (`self.Right Starting Rotation`)))
  (`GameplayStatics.PlaySoundAtLocation` "/Game/AGContent/SFX/Level/dooropenfast.dooropenfast" (`self.K2_GetActorLocation`) (struct) 1.0 1.0 0.0 null null null null)
  (bind (_direction _left_door_rotation) (`Timeline|OPen Door Timeline` :!via `PlayFromStart`)
    (:`Update`
      (`SceneComponent.K2_SetRelativeRotation` (`self.S_Wardrobe_Door_L`) (`KismetMathLibrary.MakeRotator` _left_starting_rotation_roll _left_starting_rotation_pitch _left_door_rotation) false false)
      (`SceneComponent.K2_SetRelativeRotation` (`self.S_Wardrobe_Door_R`) (`KismetMathLibrary.MakeRotator` _right_starting_rotation_roll _right_starting_rotation_pitch (* _left_door_rotation -1.0)) false false))
    (:`Finished`
      (`self.Slow Close Doors`))))

(event `Slow Close Doors`
  (bind (_left_starting_rotation_roll _left_starting_rotation_pitch) (`KismetMathLibrary.BreakRotator` (`self.Left Starting Rotation`)))
  (bind (_right_starting_rotation_roll _right_starting_rotation_pitch) (`KismetMathLibrary.BreakRotator` (`self.Right Starting Rotation`)))
  (`GameplayStatics.PlaySoundAtLocation` "/Game/AGContent/SFX/Level/DoorCreak.DoorCreak" (`self.K2_GetActorLocation`) (struct) 1.0 1.0 0.0 null null null null)
  (bind (_direction _left_door_rotation) (`Timeline|Close Door Timeline`)
    (:`Update`
      (`SceneComponent.K2_SetRelativeRotation` (`self.S_Wardrobe_Door_L`) (`KismetMathLibrary.MakeRotator` _left_starting_rotation_roll _left_starting_rotation_pitch _left_door_rotation) false false)
      (`SceneComponent.K2_SetRelativeRotation` (`self.S_Wardrobe_Door_R`) (`KismetMathLibrary.MakeRotator` _right_starting_rotation_roll _right_starting_rotation_pitch (* _left_door_rotation -1.0)) false false))))

(fn `UserConstructionScript`)