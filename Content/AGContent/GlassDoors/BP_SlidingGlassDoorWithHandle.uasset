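; Sliding double glass door actor that opens when something enters its collision box after the level is complete.
; BeginPlay caches both door meshes' world locations, and an overlap with IsLevelComplete set latches ShouldOpenDoors.
; Tick then calls MoveDoors, which slides the meshes apart along world Y at constant speed with VInterpToConstant.
; The offsets ignore actor rotation, and no logic here closes the doors or sets IsLevelComplete.
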(event `self.ReceiveBeginPlay`
  (set `self.LeftDoorWorldLocation` (`SceneComponent.K2_GetComponentLocation` (`self.LeftDoorMesh`)))
  (set `self.RightDoorWorldLocation` (`SceneComponent.K2_GetComponentLocation` (`self.RightDoorMesh`))))

(event `self.ReceiveTick`
  (params (DeltaSeconds :type "Float (single-precision)"))
  (if (`self.ShouldOpenDoors`)
    (`self.MoveDoors` DeltaSeconds)))

(event `self.CollisionBox.OnComponentBeginOverlap`
  (params (OverlappedComponent :type "PrimitiveComponent Object Reference") (OtherActor :type "Actor Object Reference") (OtherComp :type "PrimitiveComponent Object Reference") (OtherBodyIndex :type Integer) (bFromSweep :type Boolean) (SweepResult :type "HitResult Structure (by ref)"))
  (if (`self.IsLevelComplete`)
    (set `self.ShouldOpenDoors` true)))

(fn `MoveDoors`
  (params (DeltaTime :type "Float (single-precision)"))
  (locals (NewLocalVar :type "Float (single-precision)"))
  (`SceneComponent.K2_SetWorldLocation` (`self.LeftDoorMesh`) (`KismetMathLibrary.VInterpTo_Constant` (`SceneComponent.K2_GetComponentLocation` (`self.LeftDoorMesh`)) (+ (`self.LeftDoorWorldLocation`) (0.0 -150.0 0.0)) (`local.DeltaTime`) 50.0) false false)
  (`SceneComponent.K2_SetWorldLocation` (`self.RightDoorMesh`) (`KismetMathLibrary.VInterpTo_Constant` (`SceneComponent.K2_GetComponentLocation` (`self.RightDoorMesh`)) (+ (`self.RightDoorWorldLocation`) (0.0 150.0 0.0)) (`local.DeltaTime`) 50.0) false false))

(fn `UserConstructionScript`)