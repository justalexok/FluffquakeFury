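; Enemy gameplay ability that casts a spell by commanding tagged BP_Book actors in the level against the enemy's combat target.
; Activation caches the enemy, its anim blueprint and target, then plays a random tagged attack montage.
; The montage's gameplay event saves a casting pose snapshot, sets casting flags on animation and blackboard, and makes books, capped by ability level, spin and drop with damage params.
; The ability ends when the montage completes, blends out or is stopped.
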(event `self.K2_ActivateAbility`
  (bind (_tagged_montage_animmontage _tagged_montage_montagetag) (break `TaggedMontage` (`self.Tagged Montage`)))
  (bind _tagged_montage_animmontage_2 (break `TaggedMontage` (`self.Tagged Montage`)))
  (bind _abp_enemy_base (`self.ABP Enemy Base`))
  (`self.SettingVariables`)
  ;[0.07401 0.007855 0.1545] Montage
  (bind _returnvalue (message `CombatInterface.GetAttackMontages` (`self.GetAvatarActorFromActorInfo`)))
  (set `self.Tagged Montage` (`self.GetRandomTaggedMontage` _returnvalue))
  (`AbilityTask_PlayMontageAndWait.CreatePlayMontageAndWaitProxy` "None" _tagged_montage_animmontage_2
    (:`then`
      (`AbilityTask_WaitGameplayEvent.WaitGameplayEvent` _tagged_montage_montagetag null
        (:`EventReceived`
          (`AnimInstance.SavePoseSnapshot` _abp_enemy_base "CastingPose")
          (set `/Game/Blueprints/Character/Enemy/ABP_EnemyBase.Is Casting` true _abp_enemy_base)
          (`KismetSystemLibrary.PrintString` "Is Casting!")
          (`EnemyBase.SetIsCastingBlackboard` (`self.BP Enemy Base`) true)
          (bind _outactors (`GameplayStatics.GetAllActorsOfClassWithTag` "/Game/Blueprints/Actor/EffectActors/BP_Book.BP_Book_C" "Book"))
          (for (_array_element _array_index) _outactors
            (if (< _array_index (`self.GetAbilityLevel`))
              (bind _output_get (set `self.BP_Book` _array_element))
              (`/Game/Blueprints/Actor/EffectActors/BP_Book.SpinAndDrop` _output_get (`self.GetAvatarActorFromActorInfo`))
              (set `/Game/Blueprints/Actor/EffectActors/BP_Book.DamageEffectParams` (`self.MakeDamageEffectParamsFromClassDefaults` (`self.TargetActor`)) (`self.BP_Book`)))))))
    (:`OnCompleted`
      (`self.K2_EndAbility` :!label _label))
    (:`OnBlendOut`
      (goto _label))
    (:`OnInterrupted`
      (goto _label))
    (:`OnCancelled`
      (goto _label))))

(fn `SettingVariables`
  (bind _asbp_enemy_base (cast `/Game/Blueprints/Character/Enemy/BP_EnemyBase` (`self.GetAvatarActorFromActorInfo`)))
  (bind _output_get (set `self.BP Enemy Base` _asbp_enemy_base))
  (bind _asabp_enemy_base (cast `/Game/Blueprints/Character/Enemy/ABP_EnemyBase` (`SkeletalMeshComponent.GetAnimInstance` (`Character.Mesh` _output_get))))
  (set `self.ABP Enemy Base` _asabp_enemy_base)
  (bind _returnvalue (message `EnemyInterface.GetCombatTarget` (`self.BP Enemy Base`)))
  (set `self.TargetActor` _returnvalue))