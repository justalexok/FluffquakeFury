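; GA_PoisonPillowThrow is a gameplay ability that applies its default damage effect to Pippa and the enemies sharing her hotel state.
; On activation it reads the avatar's hotel state message, gathers enemies in that same state and adds the avatar itself to the targets.
; It applies damage params built from class defaults to each target, then ends immediately, with no throw or projectile logic in the graph.
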(event `self.K2_ActivateAbility`
  (`KismetSystemLibrary.PrintString` "Activated Poison Pillow THrow")
  (bind _hotel_state (message `/Game/Blueprints/Interfaces/BPI_PlayerInterface.GetPippaHotelState` (`self.GetAvatarActorFromActorInfo`)))
  (bind _enemies (`/Game/Blueprints/CommonFunctions.GetEnemiesInSameStateAsPippa` _hotel_state))
  (bind _output_get (set `self.ActorsToPoison` _enemies))
  (`KismetArrayLibrary.Array_Add` _output_get (`self.GetAvatarActorFromActorInfo`))
  (for _array_element (`self.ActorsToPoison`)
    (`FQFBlueprintFunctionLibrary.ApplyDamageEffect` (`self.MakeDamageEffectParamsFromClassDefaults` _array_element)))
  (`self.K2_EndAbility`))