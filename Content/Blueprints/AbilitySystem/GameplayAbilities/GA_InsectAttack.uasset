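; GA_InsectAttack is a gameplay ability that latches an insect enemy onto Pippa and damages her.
; On activation it casts the avatar to BP_EnemyBase and its combat target to BP_PippaCharacter.
; It activates the enemy's audio, attaches it to a random socket on Pippa's mesh at its current world transform, applies the class-default damage effect and disables movement.
; The graph never calls EndAbility.
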(event `self.K2_ActivateAbility`
  ;[0.4149 0 0.3275] Set Variables
  (bind _asbp_enemy_base (cast `/Game/Blueprints/Character/Enemy/BP_EnemyBase` (`self.GetAvatarActorFromActorInfo`)))
  (bind _output_get (set `self.BP Enemy Base` _asbp_enemy_base))
  (bind _returnvalue (message `EnemyInterface.GetCombatTarget` _output_get))
  (bind _asbp_pippa_character (cast `/Game/Blueprints/Character/Pippa/BP_PippaCharacter` _returnvalue))
  (set `self.BP Pippa Character` _asbp_pippa_character)
  (`ActorComponent.Activate` (`FQFCharacterBase.AudioComponent` (`self.BP Enemy Base`)) false)
  (`Actor.K2_AttachToComponent` (`self.BP Enemy Base`) (`Character.Mesh` (`self.BP Pippa Character`)) (`KismetArrayLibrary.Array_Random` (`self.SocketNames`)) "KeepWorld" "KeepWorld" "KeepWorld" false)
  (`FQFBlueprintFunctionLibrary.ApplyDamageEffect` (`self.MakeDamageEffectParamsFromClassDefaults` (`self.BP Pippa Character`)))
  (`CharacterMovementComponent.DisableMovement` (`Character.CharacterMovement` (`self.BP Enemy Base`))))