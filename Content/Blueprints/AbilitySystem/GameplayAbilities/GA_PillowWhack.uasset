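; Melee gameplay ability, Pillow Whack, that swings toward the point under the mouse and damages nearby live combatants.
; Stores the mouse target location, turns the avatar via CombatInterface and plays a great sword attack montage.
; A montage gameplay event triggers a small sphere query at the tagged combat socket, excluding the avatar.
; It applies damage to each actor found, then ends the ability.
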(event `self.K2_ActivateAbility`
  (bind _returnvalue (`self.GetAvatarActorFromActorInfo`))
  (`|ExecutionSequence`
    (:`then_0`
      (bind (_asynctaskproxy _datahandle) (`TargetDataUnderMouse.CreateTargetDataUnderMouse`)
        (:`ValidData`
          (bind _output_get (set `self.TargetLocation` (`.Location` (`GameplayStatics.BreakHitResult` (`AbilitySystemBlueprintLibrary.GetHitResultFromTargetData` _datahandle)))))
          (set `self.DamageImpactLocation` _output_get)
          (set `self.MouseHitActor` null))))
    (:`then_1`
      (bind _ascombat_interface (cast `CombatInterface` (`self.GetAvatarActorFromActorInfo`)))
      (`CombatInterface.SetFacingTarget` _ascombat_interface (`self.TargetLocation`))
      (`AbilityTask_PlayMontageAndWait.CreatePlayMontageAndWaitProxy` "None" "/Game/AGContent/Characters/Mixamo/Timmy/Animations/AM_GreatSwordAttack.AM_GreatSwordAttack"
        (:`then`
          (`AbilityTask_WaitGameplayEvent.WaitGameplayEvent` (`self.Event Tag`) null
            (:`EventReceived`
              (bind _returnvalue_2 (message `CombatInterface.GetCombatSocketLocation` _returnvalue (`self.Event Tag`)))
              (bind _outoverlappingactors (`FQFBlueprintFunctionLibrary.GetLivePlayersWithinRadius` _returnvalue (`|MakeArray` _returnvalue) 22.5 _returnvalue_2))
              (for _array_element _outoverlappingactors
                (bind _output_get_2 (set `self.TargetActor` _array_element))
                (`self.ApplyDamageToTargetActor` _output_get_2))
              (`self.K2_EndAbility`))))))))

(event `self.K2_OnEndAbility`
  (params (bWasCancelled :type Boolean)))