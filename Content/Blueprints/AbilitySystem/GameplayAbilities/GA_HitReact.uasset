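; GA_HitReact is the gameplay ability that plays an avatar's hit reaction.
; On activation it applies GE_HitReact to the owner, then plays the montage supplied by the avatar's CombatInterface at increased rate.
; It calls SetMaxWalkSpeed(true) as the montage starts and SetMaxWalkSpeed(false) only on blend out.
; Completion, interruption or cancellation removes the effect by its stored handle and ends the ability.
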(event `self.K2_ActivateAbility`
  (bind _returnvalue (`self.BP_ApplyGameplayEffectToOwner` "/Game/Blueprints/AbilitySystem/GameplayEffects/GE_HitReact.GE_HitReact_C"))
  (set `self.Active GE Hit React` _returnvalue)
  (bind _ascombat_interface (cast `CombatInterface` (`self.GetAvatarActorFromActorInfo`)))
  (bind _output_get (set `self.Combat Interface` _ascombat_interface))
  (bind _returnvalue_2 (`CombatInterface.GetHitReactMontage` _output_get))
  (`AbilityTask_PlayMontageAndWait.CreatePlayMontageAndWaitProxy` "None" _returnvalue_2 2.0
    (:`then`
      (`CombatInterface.SetMaxWalkSpeed` (`self.Combat Interface`) true))
    (:`OnCompleted`
      (`self.BP_RemoveGameplayEffectFromOwnerWithHandle` (`self.Active GE Hit React`) :!label _label)
      (`self.K2_EndAbility`))
    (:`OnBlendOut`
      (`CombatInterface.SetMaxWalkSpeed` (`self.Combat Interface`) false))
    (:`OnInterrupted`
      (goto _label))
    (:`OnCancelled`
      (goto _label))))