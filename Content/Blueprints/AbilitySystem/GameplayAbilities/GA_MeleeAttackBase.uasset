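; Base melee attack gameplay ability for enemies, which faces the combat target and picks a random attack tag from the owning BP_EnemyBase.
; The tag looks up ability info for the montage, event tag and damage curve.
; On the montage's gameplay event, it damages live players around the combat socket, shakes the camera and ends.
; A tag-based knockback function exists but is not wired into the running flow.
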(event `self.K2_ActivateAbility`
  (bind _returnvalue (`self.GetAvatarActorFromActorInfo`))
  (bind _returnvalue_2 (`self.GetAvatarActorFromActorInfo`))
  (bind (_abilityinfo_abilitytag _abilityinfo_gameplayability _abilityinfo_montagetag) (break `FQFAbilityInfo` (`self.AbilityInfo`)))
  (bind (_abilityinfo_abilitytag_2 _abilityinfo_gameplayability_2 _abilityinfo_montagetag_2 _abilityinfo_animmontage _abilityinfo_sockettagname _abilityinfo_busesweapon _abilityinfo_inputtag _abilityinfo_damagecurve) (break `FQFAbilityInfo` (`self.AbilityInfo`)))
  ;[0.07401 0.007855 0.1545] Face Target
  (bind _returnvalue_3 (message `EnemyInterface.GetCombatTarget` _returnvalue))
  (message `CombatInterface.SetFacingTarget` _returnvalue (`Actor.K2_GetActorLocation` _returnvalue_3))
  (`self.SetSpecificAbilityTag`)
  ;[0.002408 0.1007 0.03194] Get Ability Info
  (bind _returnvalue_4 (`FQFBlueprintFunctionLibrary.GetAbilityInfo` (`self.GetAvatarActorFromActorInfo`)))
  (bind _output_get (set `self.AbilityInfo` (`AbilityInfo.FindAbilityInfoForTag` _returnvalue_4 (`self.SpecificAbilityTag`) false)))
  (`AbilityTask_PlayMontageAndWait.CreatePlayMontageAndWaitProxy` "None" (`.AnimMontage` (break `FQFAbilityInfo` _output_get))
    (:`then`
      (`AbilityTask_WaitGameplayEvent.WaitGameplayEvent` _abilityinfo_montagetag null
        (:`EventReceived`
          (set `self.Damage` _abilityinfo_damagecurve)
          (set `self.OwnerFowardVector` (`Actor.GetActorForwardVector` (`self.GetAvatarActorFromActorInfo`)))
          (bind _returnvalue_5 (message `CombatInterface.GetCombatSocketLocation` (`self.GetAvatarActorFromActorInfo`) (`self.SpecificAbilityTag`)))
          (bind _outoverlappingactors (`FQFBlueprintFunctionLibrary.GetLivePlayersWithinRadius` _returnvalue_2 (`|MakeArray` _returnvalue_2) 22.5 _returnvalue_5))
          (for _array_element _outoverlappingactors
            (bind _output_get_2 (set `self.HitActor` _array_element))
            (`FQFBlueprintFunctionLibrary.ApplyDamageEffect` (`self.MakeDamageEffectParamsFromClassDefaults` _output_get_2))
            (`GameplayStatics.PlayWorldCameraShake` "/Game/Blueprints/Game/BP_Low_CameraShake.BP_Low_CameraShake_C" (`Actor.K2_GetActorLocation` _output_get_2) 0.0 500.0))
          (`self.K2_EndAbility`))))
    (:`OnCompleted`
      (`self.K2_EndAbility` :!label _label))
    (:`OnInterrupted`
      (goto _label))
    (:`OnCancelled`
      (goto _label))))

(fn `KnockbackIfApplicable`
  (bind _abilityinfo_abilitytag (break `FQFAbilityInfo` (`self.AbilityInfo`)))
  (bind _abilityinfo_abilitytag_2 (break `FQFAbilityInfo` (`self.AbilityInfo`)))
  (if (`BlueprintGameplayTagLibrary.MatchesTag` _abilityinfo_abilitytag (struct :`TagName` "Abilities.Squash"))
    (message `CombatInterface.KnockbackCharacter` (`self.HitActor`) 350.0 45.0 (`self.OwnerFowardVector`))
    (elif (`BlueprintGameplayTagLibrary.MatchesTag` _abilityinfo_abilitytag_2 (struct :`TagName` "Abilities.TwoHandedJumpAttack"))
      (message `CombatInterface.KnockbackCharacter` (`self.HitActor`) 100.0 45.0 (`self.OwnerFowardVector`)))))

(fn `SetSpecificAbilityTag`
  (bind _asbp_enemy_base (cast `/Game/Blueprints/Character/Enemy/BP_EnemyBase` (`self.GetAvatarActorFromActorInfo`)))
  (set `self.SpecificAbilityTag` (`KismetArrayLibrary.Array_Random` (`EnemyBase.SpecificAbilityTags` _asbp_enemy_base))))