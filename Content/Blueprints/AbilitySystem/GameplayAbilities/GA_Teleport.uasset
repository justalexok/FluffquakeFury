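; Gameplay ability that teleports the AI-driven Jolleen character behind a montage.
; On activation it sets HasBeenHit on Jolleen's AnimBP and the AmITeleporting blackboard flag through CombatInterface, then plays AM_Teleport.
; On montage blend out it saves a TeleportingPose snapshot in the AnimBP and calls TeleportActor on the character.
; The ability never calls EndAbility or clears either flag itself.
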(event `self.K2_ActivateAbility`
  (`self.Set Variables`)
  (`AbilityTask_PlayMontageAndWait.CreatePlayMontageAndWaitProxy` "None" "/Game/AGContent/Characters/Mixamo/Jolleen/Animations/AM_Teleport.AM_Teleport"
    (:`OnBlendOut`
      (`AnimInstance.SavePoseSnapshot` (`self.ABP Jolleen`) "TeleportingPose")
      (bind _asbp_jolleen (cast `/Game/Blueprints/Character/Enemy/Jolleen/BP_Jolleen` (`self.GetAvatarActorFromActorInfo`)))
      (`/Game/Blueprints/Character/Enemy/Jolleen/BP_Jolleen.Teleport Actor` _asbp_jolleen))))

(fn `Set Variables`
  (bind _ascombat_interface (cast `CombatInterface` (`self.GetAvatarActorFromActorInfo`)))
  (bind _output_get (set `self.Combat Interface` _ascombat_interface))
  (bind _returnvalue (`CombatInterface.GetAnimInstance` _output_get))
  (bind _asabp_jolleen (cast `/Game/Blueprints/Character/Enemy/Jolleen/ABP_Jolleen` _returnvalue))
  (bind _output_get_2 (set `self.ABP Jolleen` _asabp_jolleen))
  (set `/Game/Blueprints/Character/Enemy/Jolleen/ABP_Jolleen.HasBeenHit` true _output_get_2)
  (`CombatInterface.SetBlackboardBoolForKey` (`self.Combat Interface`) "AmITeleporting" true))