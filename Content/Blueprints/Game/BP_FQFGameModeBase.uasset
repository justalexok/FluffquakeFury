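; Game mode that runs level failure and completion flow and spawns enemies.
; Player death broadcasts level failure, which shows a timed retry widget, then restarts the current world.
; Level completion stops spawning and broadcasts world completion on the world's last level.
; A looping timer, cleared after a computed delay, spawns enemies at random collection points (navigable-radius placement also supported), adding colored Niagara effects and level-index tags.
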(event `OnLevelFailureDelegate_Event`
  ;[0.6615 0 0.04132] On Level Fail
  (`GameplayStatics.PlaySound2D` "/Game/AGContent/SFX/Level/LevelFail.LevelFail" 1.0 1.0 0.0 null null)
  (bind _returnvalue (`|CreateWidget` "/Game/Blueprints/UI/LevelWidgets/WBP_RetryLevel.WBP_RetryLevel_C"))
  (`UserWidget.AddToViewport` _returnvalue 0)
  (`KismetSystemLibrary.Delay` (`KismetMathLibrary.Conv_IntToDouble` (`/Game/Blueprints/UI/LevelWidgets/WBP_RetryLevel.TimerValue` _returnvalue)))
  (`self.RestartCurrentWorld`))

(event `self.ReceiveBeginPlay`
  (bind _aspippa_player_controller (cast `PippaPlayerController` (`GameplayStatics.GetPlayerController` 0)))
  (set `self.Pippa Player Controller` _aspippa_player_controller)
  (`|ExecutionSequence`
    (:`then_0`
      ;[0.6615 0 0.04132] On Level Fail
      (add `PippaPlayerController.OnLevelFailureDelegate` (`self.Pippa Player Controller`) (delegate `OnLevelFailureDelegate_Event`))
      (add `self.OnLevelFailureDelegate` (delegate `OnLevelFailureDelegate_Event`)))
    (:`then_1`
      ;[0.2448 0 0.0218] On Player Death
      (add `self.OnPlayerDeathDelegate` (delegate `OnPlayerDeathDelegate_Event`)))
    (:`then_2`
      ;[0 0.276 0.1044] On Level Complete
      (add `self.OnLevelCompletionDelegate` (delegate `OnLevelCompletionDelegate_Event`)))))

(event `OnPlayerDeathDelegate_Event`
  ;[0.2448 0 0.0218] On Player Death
  (`self.BroadcastLevelFailure`))

(event `OnLevelCompletionDelegate_Event`
  ;[0 0.276 0.1044] On Level Complete
  (`GameplayStatics.PlaySound2D` "/Game/AGContent/SFX/Level/LevelComplete.LevelComplete" 1.0 1.0 0.0 null null)
  (`KismetSystemLibrary.K2_ClearAndInvalidateTimerHandle` (`self.SpawnTimerHandle`))
  (bind _is_world_complete (`self.CalculateIfWorldComplete`))
  (if _is_world_complete
    (`self.BroadcastWorldCompletion`)))

(event `SpawnEnemy`
  (params (FromPointCollection :type Boolean) (EnemyClass :type "Actor Class Reference"))
  ;[0 0.09282 0.09896] Spawn Enemies
  (set `self.Enemy Class` EnemyClass)
  (if FromPointCollection
    (bind _spawntransform (`self.GetSpawnTransformFromPoints`))
    (bind _returnvalue (`|SpawnActorFromClass` (`self.Enemy Class`) _spawntransform "AdjustIfPossibleButDontSpawnIfColliding" "MultiplyWithRoot" null null))
    (`self.Handle Spawn` _returnvalue)
    (else
      (bind _spawntransform_2 (`self.Get Spawn Transform in Navigable Radius`))
      (bind _returnvalue_2 (`|SpawnActorFromClass` (`self.Enemy Class`) _spawntransform_2 "AdjustIfPossibleButDontSpawnIfColliding" "MultiplyWithRoot" null null))
      (`self.Handle Spawn` _returnvalue_2))))

(event `BeginSpawnSequence`
  (params (SpawnFrequency :type "Float (double-precision)") (DesiredEnemyCount :type "Float (double-precision)"))
  ;[0 0.09282 0.09896] Spawn Enemies
  (bind _returnvalue (`KismetSystemLibrary.K2_SetTimerDelegate` (delegate `TimedSpawn`) (`self.SpawnFrequency`) true))
  (set `self.SpawnTimerHandle` _returnvalue)
  (`KismetSystemLibrary.Delay` (* (`self.SpawnFrequency`) (+ (`self.DesiredEnemyCount`) 1.0)))
  (`KismetSystemLibrary.K2_ClearAndInvalidateTimerHandle` (`self.SpawnTimerHandle`)))

(event `TimedSpawn`
  ;[0 0.09282 0.09896] Spawn Enemies
  (`self.SpawnEnemy` true (`self.Enemy Class`)))

(fn `CalculateIfWorldComplete`
  (returns (`Is World Complete` :type Boolean))
  (bind _returnvalue (`self.CountNumLevelsInCurrentWorld`))
  (bind _returnvalue_2 (`self.GetCurrentLevelInfo`))
  (return (== _returnvalue (break `FQFLevelInfo` _returnvalue_2))))

(fn `Get Spawn Transform in Navigable Radius`
  (returns (SpawnTransform :type "Transform Structure"))
  (locals (Origin :type "Vector Structure" :default (0.0 0.0 0.0)))
  (return (`KismetMathLibrary.MakeTransform` (`NavigationSystemV1.K2_GetRandomReachablePointInRadius` (`local.Origin`) 1000.0 null null) (struct :`Yaw` 180.0))))

(fn `GetSpawnTransformFromPoints`
  (returns (SpawnTransform :type "Transform Structure"))
  (bind _returnvalue (`GameplayStatics.GetActorOfClass` "/Game/Blueprints/Actor/SpawnPoints/BP_L1_SpawnPoints.BP_L1_SpawnPoints_C"))
  (bind _output_get (set `self.SpawnPointsCollection` _returnvalue))
  (return (`KismetMathLibrary.MakeTransform` (`SceneComponent.K2_GetComponentLocation` (`KismetArrayLibrary.Array_Random` (`/Game/Blueprints/Actor/SpawnPoints/BP_L1_SpawnPoints.SpawnPoints` _output_get))) (struct :`Yaw` 180.0))))

(fn `Handle Spawn`
  (params (Object :type "Object Object Reference"))
  (bind _asbp_enemy_base (cast `/Game/Blueprints/Character/Enemy/BP_EnemyBase` Object))
  (bind _output_get (set `self.Spawned Enemy` _asbp_enemy_base))
  (`/Engine/EditorBlueprintResources/StandardMacros.IsValid` _output_get
    (:`Is Valid`
      (`self.SpawnNiagara` _output_get)
      (`self.SetEnemyTagForLevel` _output_get))))

(fn `SetEnemyTagForLevel`
  (params (Enemy :type "Actor Object Reference"))
  (bind _returnvalue (`self.GetCurrentLevelInfo`))
  (bind _output_get (set `self.LevelTag` (`KismetStringLibrary.Conv_StringToName` (`KismetStringLibrary.Conv_IntToString` (break `FQFLevelInfo` _returnvalue)))))
  (set `Actor.Tags` (`|MakeArray` _output_get) Enemy))

(fn `SpawnNiagara`
  (params (Enemy :type "/Game/Blueprints/Character/Enemy/BP_EnemyBase Object Reference"))
  (bind _returnvalue (`FQFBlueprintFunctionLibrary.SpawnNiagaraAtPoint` Enemy (0.0 0.0 0.0) Enemy "Ground" (1.0 1.0 1.0) "/Game/AGContent/Niagara/NS_PickupSet/Fx/NiagaraSystems/NS_CharacterSpawn.NS_CharacterSpawn"))
  (`NiagaraComponent.SetVariableLinearColor` _returnvalue "Color01" (`FQFCharacterBase.CharacterColor` Enemy))
  (`NiagaraComponent.SetVariableFloat` _returnvalue "Lifetime" 1.0))

(fn `UserConstructionScript`)