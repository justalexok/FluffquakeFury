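; CommonFunctions is a Blueprint of shared helper functions for on-screen hit messages and enemy queries.
; CreateFloatingTextWidget spawns a WBP_FloatingText, blanks its damage text, shows the given message, plays the hit message animation and adds it to the viewport.
; GetEnemiesInSameStateAsPippa scans every BP_EnemyBase actor in the world and returns those whose HotelState matches the Pippa hotel state passed in.
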(fn `Create Floating Text Widget`
  (params (Message :type Name))
  (bind _returnvalue (`|CreateWidget` "/Game/Blueprints/UI/FloatingText/WBP_FloatingText.WBP_FloatingText_C"))
  (`TextBlock.SetText` (`/Game/Blueprints/UI/FloatingText/WBP_FloatingText.Text_DamageAmount` _returnvalue) "")
  (`TextBlock.SetText` (`/Game/Blueprints/UI/FloatingText/WBP_FloatingText.Text_HitMessage` _returnvalue) (`KismetTextLibrary.Conv_NameToText` Message))
  (`UserWidget.PlayAnimation` _returnvalue (`/Game/Blueprints/UI/FloatingText/WBP_FloatingText.HitMessageAnim` _returnvalue) 0.0 1 "Forward" 1.0 false)
  (`UserWidget.AddToViewport` _returnvalue 0))

(fn `GetEnemiesInSameStateAsPippa`
  (params (`Pippa Hotel State` :type "/Game/Blueprints/Game/HotelState Enum" :default "NewEnumerator0"))
  (returns (Enemies :type "Array of /Game/Blueprints/Character/Enemy/BP_EnemyBase Object Reference"))
  (locals (EnemiesToReturn :type "Array of /Game/Blueprints/Character/Enemy/BP_EnemyBase Object Reference"))
  (bind _outactors (`GameplayStatics.GetAllActorsOfClass` null "/Game/Blueprints/Character/Enemy/BP_EnemyBase.BP_EnemyBase_C"))
  (for _array_element _outactors
    (if (`|EnumEquality` `Pippa Hotel State` (`/Game/Blueprints/Character/Enemy/BP_EnemyBase.HotelState` _array_element))
      (`KismetArrayLibrary.Array_Add` (`local.EnemiesToReturn`) _array_element)))
  (return (`local.EnemiesToReturn`)))