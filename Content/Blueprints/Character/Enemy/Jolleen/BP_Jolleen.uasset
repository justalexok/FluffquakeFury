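; Jolleen enemy character whose TeleportActor event relocates it and raises its enemy level on each call.
; A Sequence overlaps delayed phases: a timeline lifts it from a green Niagara magic circle while a new random point is picked from BP_JolleenSPCollection.
; Unless it is dead, a reversed timeline lowers it there, then clears the blackboard teleport flag and animation states and faces the player.
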(event `Teleport Actor`
  (`|ExecutionSequence`
    (:`then_0`
      (bind _ascombat_interface (cast `CombatInterface` self))
      (set `self.Combat Interface` _ascombat_interface)
      (`GameplayStatics.PlaySoundAtLocation` "/Game/AGContent/SFX/Misc/Teleport.Teleport" (`self.K2_GetActorLocation`) (struct) 1.0 1.0 0.0 null null null null)
      (`KismetSystemLibrary.Delay` 0.35)
      ;[0.5271 0.07227 0.05448] Eject Niagara
      (if (not (`CombatInterface.IsDead` (`self.Combat Interface`)))
        (bind _returnvalue (`FQFBlueprintFunctionLibrary.SpawnNiagaraAtPoint` self (0.0 0.0 0.0) self "Ground" (`self.TeleportNiagaraScal`) "/Game/AGContent/Niagara/FXVarietyPack/Particles/NS_GreenMagicCircle.NS_GreenMagicCircle"))
        ;[0.2135 0 0.01994] Eject
        (bind (_direction _zlocationfloat) (`Timeline|Eject Timeline` :!via `PlayFromStart`)
          (:`Update`
            (`self.K2_SetActorLocation` (+ (`self.K2_GetActorLocation`) (`KismetMathLibrary.MakeVector` 0.0 0.0 _zlocationfloat))))
          (:`Finished`
            (`ActorComponent.K2_DestroyComponent` _returnvalue)))))
    (:`then_1`
      ;[0.07401 0.007855 0.1545] Get Next Location
      (`KismetSystemLibrary.Delay` 0.5)
      (bind _returnvalue_2 (`GameplayStatics.GetActorOfClass` "/Game/Blueprints/Actor/SpawnPoints/MainBedroom/BP_JolleenSPCollection.BP_JolleenSPCollection_C"))
      (bind _output_get (set `self.PointCollection` _returnvalue_2))
      (set `self.Jolleen Next Location` (+ (`PointCollection.GetRandomNewGroundPoint` _output_get (- (`self.Jolleen Next Location`) (`KismetMathLibrary.MakeVector` 0.0 0.0 (`CapsuleComponent.CapsuleHalfHeight` (`self.CapsuleComponent`)))) 0.0) (`KismetMathLibrary.MakeVector` 0.0 0.0 (`CapsuleComponent.CapsuleHalfHeight` (`self.CapsuleComponent`)))))
      ;[0.5271 0.07227 0.05448] Return Niagara
      (if (not (`CombatInterface.IsDead` (`self.Combat Interface`)))
        (bind _returnvalue_3 (`FQFBlueprintFunctionLibrary.SpawnNiagaraAtPoint` self (- (`self.Jolleen Next Location`) (`KismetMathLibrary.MakeVector` 0.0 0.0 (`CapsuleComponent.CapsuleHalfHeight` (`self.CapsuleComponent`)))) null "Center" (`self.TeleportNiagaraScal`) "/Game/AGContent/Niagara/FXVarietyPack/Particles/NS_GreenMagicCircle.NS_GreenMagicCircle"))
        (set `self.MagicCircleNiagara` _returnvalue_3)
        ;[0.3559 0 0.02224] Bring Down Actor
        (bind (_direction_2 _zlocationfloat_2) (`Timeline|Timeline_1` :!via `ReverseFromEnd`)
          (:`Update`
            (`self.K2_SetActorLocation` (+ (`self.Jolleen Next Location`) (`KismetMathLibrary.MakeVector` 0.0 0.0 _zlocationfloat_2))))
          (:`Finished`
            ;[0 0.08265 0.1024] Set Variables
            (`CombatInterface.SetBlackboardBoolForKey` "AmITeleporting")
            (bind _returnvalue_4 (`CombatInterface.GetAnimInstance` (`self.Combat Interface`)))
            (bind _asabp_jolleen (cast `/Game/Blueprints/Character/Enemy/Jolleen/ABP_Jolleen` _returnvalue_4))
            (set `/Game/Blueprints/Character/Enemy/Jolleen/ABP_Jolleen.IsCasting` false _asabp_jolleen)
            (set `/Game/Blueprints/Character/Enemy/Jolleen/ABP_Jolleen.HasBeenHit` false _asabp_jolleen)
            (`CombatInterface.SetFacingTarget` (`self.Combat Interface`) (`self.K2_GetActorLocation` (`Controller.K2_GetPawn` (`GameplayStatics.GetPlayerController` 0))))
            (`KismetSystemLibrary.Delay` 1.5)
            (`ActorComponent.K2_DestroyComponent` (`self.MagicCircleNiagara`))))))
    (:`then_2`
      (`self.IncrementEnemyLevel`))))

(event `self.ReceiveBeginPlay`
  (`parent.ReceiveBeginPlay`)
  (set `self.Jolleen Starting Location` (`self.K2_GetActorLocation`)))

(event `self.ReceiveTick`
  (params (DeltaSeconds :type "Float (single-precision)"))
  (`parent.ReceiveTick` DeltaSeconds))

(fn `UserConstructionScript`
  (`parent.UserConstructionScript`))