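; Slime monster enemy Blueprint that adds a timed defend behavior and starts its audio component on BeginPlay.
; Defend raises the defending state, attaches a Niagara halo above the mesh, growls partway through, then clears both after fixed delays.
; SetIsDefending mirrors the flag to the slime's Animation Blueprint and sends it to the AmIDefending Blackboard key through a message call, syncing animation and AI.
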(event `self.ReceiveBeginPlay`
  (`parent.ReceiveBeginPlay`)
  (`ActorComponent.Activate` (`self.AudioComponent`) false))

(event `Defend`
  (`self.SetIsDefending` true)
  (bind _mesh (`self.Mesh`)
    (:`then`
      (bind _returnvalue (`NiagaraFunctionLibrary.SpawnSystemAttached` "/Game/AGContent/Niagara/NS_Halo.NS_Halo" _mesh "None" (0.0 0.0 100.0) (struct) "KeepRelativeOffset" true))
      (set `self.NS Halo` _returnvalue)
      (`KismetSystemLibrary.Delay` 1.5)
      (`GameplayStatics.PlaySoundAtLocation` "/Game/AGContent/SFX/HitReacts/MonsterGrowl.MonsterGrowl" (`self.K2_GetActorLocation`) (struct) 1.0 1.0 0.0 null null null null)
      (`KismetSystemLibrary.Delay` 4.5)
      (`ActorComponent.Deactivate` (`self.NS Halo`))
      (`self.SetIsDefending` false))
    (:`else`)))

(fn `SetIsDefending`
  (params (` Is Defending` :type Boolean))
  (locals (`L Is Defending` :type Boolean))
  (set `local.L Is Defending` ` Is Defending`)
  (bind _returnvalue (`CombatInterface.GetAnimInstance`))
  (bind _asabp_slime_monster (cast `/Game/Blueprints/Character/Enemy/SlimeMonster/ABP_SlimeMonster` _returnvalue))
  (bind _output_get (set `self.ABP Slime Monster` _asabp_slime_monster))
  (set `/Game/Blueprints/Character/Enemy/SlimeMonster/ABP_SlimeMonster.IsDefending` (`local.L Is Defending`) _output_get)
  (message `CombatInterface.SetBlackboardBoolForKey` self "AmIDefending" (`local.L Is Defending`)))

(fn `UserConstructionScript`
  (`parent.UserConstructionScript`))