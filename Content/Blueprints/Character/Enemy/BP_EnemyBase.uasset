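; Base enemy character Blueprint that handles spawn, facing and dissolve presentation.
; On BeginPlay a timeline scales the mesh relative to its initial scale.
; Facing events either interpolate rotation toward the player pawn in a single step or update the "FacingTarget" Motion Warping target from a location.
; Separate body and weapon timelines drive the "Dissolve" parameter on dynamic material instances passed into their events.
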(event `self.ReceiveBeginPlay`
  (set `self.InitialMeshScale` (`SceneComponent.RelativeScale3D` (`self.Mesh`)))
  (bind (_direction _scaletrack) (`Timeline|SpawnTimeline`)
    (:`Update`
      (`SceneComponent.SetRelativeScale3D` (`self.Mesh`) (* (`KismetMathLibrary.MakeVector` _scaletrack _scaletrack _scaletrack) (`self.InitialMeshScale`))))))

(event `ManuallyFacePlayer`
  (`self.K2_SetActorRotation` (`KismetMathLibrary.RInterpTo` (`self.K2_GetActorRotation`) (`KismetMathLibrary.FindLookAtRotation` (`self.K2_GetActorLocation`) (`self.K2_GetActorLocation` (`GameplayStatics.GetPlayerPawn` 0))) 1.0 5.0)))

(event `CombatInterface.SetFacingTarget`
  (params (FacingTarget :type "Vector Structure (by ref)"))
  (`MotionWarpingComponent.AddOrUpdateWarpTargetFromLocation` (`self.MotionWarping`) "FacingTarget" FacingTarget))

(event `self.StartDissolveTimeline`
  (params (DynamicMaterialInstance :type "MaterialInstanceDynamic Object Reference"))
  (bind (_direction _dissolvetrack) (`Timeline|Timeline`)
    (:`Update`
      (`MaterialInstanceDynamic.SetScalarParameterValue` DynamicMaterialInstance "Dissolve" _dissolvetrack))))

(event `self.StartWeaponDissolveTimeline`
  (params (DynamicMaterialInstance :type "MaterialInstanceDynamic Object Reference"))
  (bind (_direction _dissolvetrack) (`Timeline|Timeline_0`)
    (:`Update`
      (`MaterialInstanceDynamic.SetScalarParameterValue` DynamicMaterialInstance "Dissolve" _dissolvetrack))))

(fn `UserConstructionScript`)