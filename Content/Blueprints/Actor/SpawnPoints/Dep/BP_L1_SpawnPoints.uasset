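; BP_L1_SpawnPoints is an actor that collects a fixed group of spawn points, apparently for L1.
; On BeginPlay it appends its six CenterPoint references to the SpawnPoints0 array in index order.
; It contains no spawning logic, and its Tick, overlap and construction script are empty, so it acts only as a point container.
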(event `self.ReceiveBeginPlay`
  (`KismetArrayLibrary.Array_Add` (`self.SpawnPoints_0`) (`self.CenterPoint_0`))
  (`KismetArrayLibrary.Array_Add` (`self.SpawnPoints_0`) (`self.CenterPoint1`))
  (`KismetArrayLibrary.Array_Add` (`self.SpawnPoints_0`) (`self.CenterPoint2`))
  (`KismetArrayLibrary.Array_Add` (`self.SpawnPoints_0`) (`self.CenterPoint3`))
  (`KismetArrayLibrary.Array_Add` (`self.SpawnPoints_0`) (`self.CenterPoint4`))
  (`KismetArrayLibrary.Array_Add` (`self.SpawnPoints_0`) (`self.CenterPoint5`)))

(fn `UserConstructionScript`)