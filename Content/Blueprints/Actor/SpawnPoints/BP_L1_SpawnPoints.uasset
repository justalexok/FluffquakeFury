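; BP_L1_SpawnPoints is an actor that holds a set of spawn points, apparently for level 1.
; On BeginPlay it adds five center point references to its SpawnPoints array.
; It contains no spawning logic itself; overlap, tick and the construction script do nothing.
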(event `self.ReceiveBeginPlay`
  (`KismetArrayLibrary.Array_Add` (`self.SpawnPoints`) (`self.CenterPoint`))
  (`KismetArrayLibrary.Array_Add` (`self.SpawnPoints`) (`self.CenterPoint1`))
  (`KismetArrayLibrary.Array_Add` (`self.SpawnPoints`) (`self.CenterPoint2`))
  (`KismetArrayLibrary.Array_Add` (`self.SpawnPoints`) (`self.CenterPoint3`))
  (`KismetArrayLibrary.Array_Add` (`self.SpawnPoints`) (`self.CenterPoint4`)))

(fn `UserConstructionScript`)