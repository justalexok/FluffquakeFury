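; Bed actor that serves as the exit to the next world once the world can be completed.
; TiltBed rolls the mesh on a timeline, then fires the completion dispatcher, whose bound handler enables the exit trigger, reattaches the player camera and spawns heal auras every three seconds.
; Player overlap with the trigger calls GoToNextWorld on the game mode.
; Bounce-pad launch and aura logic is disconnected and never runs.
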(event `self.ReceiveBeginPlay`
  (add `self.WorldCanBeComplete` (delegate `WorldCanBeComplete_Event`))
  (`PrimitiveComponent.SetCollisionResponseToAllChannels` (`self.NextWorldCollision`) "ECR_Ignore"))

(event `WorldCanBeComplete_Event`
  (`PrimitiveComponent.SetCollisionResponseToAllChannels` (`self.NextWorldCollision`) "ECR_Overlap")
  (`self.Spawn Niagara`)
  (message `/Game/Blueprints/Interfaces/BPI_PlayerInterface.AttachCameraToSpringArm` (`GameplayStatics.GetPlayerPawn` 0)))

(event `Spawn Niagara`
  (`|SpawnActorFromClass` "/Game/AGContent/Niagara/FXVarietyPack/Blueprints/BP_ky_healAura.BP_ky_healAura_C" (`KismetMathLibrary.Conv_VectorToTransform` (`SceneComponent.K2_GetComponentLocation` (`self.NiagaraSpawnPoint`))) "Undefined" "MultiplyWithRoot" null null :!label _label)
  (`KismetSystemLibrary.Delay` 3.0)
  (goto _label))

(event `self.NextWorldCollision.OnComponentBeginOverlap`
  (params (OverlappedComponent :type "PrimitiveComponent Object Reference") (OtherActor :type "Actor Object Reference") (OtherComp :type "PrimitiveComponent Object Reference") (OtherBodyIndex :type Integer) (bFromSweep :type Boolean) (SweepResult :type "HitResult Structure (by ref)"))
  (bind _returnvalue (`GameplayStatics.GetPlayerPawn` 0))
  (if (== OtherActor _returnvalue)
    (bind _returnvalue_2 (`FQFBlueprintFunctionLibrary.GetFQFGameMode` _returnvalue))
    (bind _asbp_fqfgame_mode_base (cast `/Game/Blueprints/Game/BP_FQFGameModeBase` _returnvalue_2))
    (`/Game/Blueprints/Game/BP_FQFGameModeBase.GoToNextWorld` _asbp_fqfgame_mode_base)))

(event `Tilt Bed`
  (bind (_direction _newtrack_0) (`Timeline|Timeline` :!via `PlayFromStart`)
    (:`Update`
      (`SceneComponent.K2_SetWorldRotation` (`self.StaticMeshComponent`) (`KismetMathLibrary.MakeRotator` _newtrack_0 0.0 -90.0) false false))
    (:`Finished`
      (`self.WorldCanBeComplete_Event`))))

(event `self.BouncePad.OnComponentBeginOverlap`
  (params (OverlappedComponent :type "PrimitiveComponent Object Reference") (OtherActor :type "Actor Object Reference") (OtherComp :type "PrimitiveComponent Object Reference") (OtherBodyIndex :type Integer) (bFromSweep :type Boolean) (SweepResult :type "HitResult Structure (by ref)"))
  ;[0.3073 0.3073 0.3073] Comment
)

(event `self.BouncingZone.OnComponentEndOverlap`
  (params (OverlappedComponent :type "PrimitiveComponent Object Reference") (OtherActor :type "Actor Object Reference") (OtherComp :type "PrimitiveComponent Object Reference") (OtherBodyIndex :type Integer))
  ;[0.3073 0.3073 0.3073] Comment
)

(fn `UserConstructionScript`)