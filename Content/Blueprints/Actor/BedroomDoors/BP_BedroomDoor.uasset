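; Bedroom door actor that moves Pippa between the landing and a room through enter and leave trigger boxes.
; On entering, it reattaches her camera to a fixed room point, teleports her inside and adds a rotate-right input mapping context.
; On leaving, it returns the camera to her spring arm, sends her to the landing and removes that context.
; Both transitions trigger a brief fade widget spawned by the game mode.
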(event `self.EnterBoxCollision.OnComponentBeginOverlap`
  (params (OverlappedComponent :type "PrimitiveComponent Object Reference") (OtherActor :type "Actor Object Reference") (OtherComp :type "PrimitiveComponent Object Reference") (OtherBodyIndex :type Integer) (bFromSweep :type Boolean) (SweepResult :type "HitResult Structure (by ref)"))
  (bind _asbp_pippa_character (cast `/Game/Blueprints/Character/Pippa/BP_PippaCharacter` OtherActor))
  (`self.Fade Widget`)
  (bind _output_get (set `self.BP Pippa Character` _asbp_pippa_character))
  ;[0.01758 0.2458 0.3142] Modify Camera
  (`SceneComponent.K2_AttachToComponent` (`PippaCharacter.Camera` _output_get) (`self.CameraPoint`) "None" "KeepRelative" "KeepRelative" "KeepRelative" true)
  ;[0.01198 0.09048 0.342] Teleport Pippa and Switch IMC
  (`self.K2_SetActorLocationAndRotation` :`self` (`self.BP Pippa Character`) :`NewLocation` (`SceneComponent.K2_GetComponentLocation` (`self.InRoomPlayerStart`)))
  (`EnhancedInputSubsystemInterface.AddMappingContext` (pcsubsystem `EnhancedInputLocalPlayerSubsystem` (`GameplayStatics.GetPlayerController` 0)) "/Game/Blueprints/Input/IMC_RotateRight_PippaContext.IMC_RotateRight_PippaContext" 0 (struct)))

(event `self.LeaveBoxCollision.OnComponentBeginOverlap`
  (params (OverlappedComponent :type "PrimitiveComponent Object Reference") (OtherActor :type "Actor Object Reference") (OtherComp :type "PrimitiveComponent Object Reference") (OtherBodyIndex :type Integer) (bFromSweep :type Boolean) (SweepResult :type "HitResult Structure (by ref)"))
  (bind _asbp_pippa_character (cast `/Game/Blueprints/Character/Pippa/BP_PippaCharacter` OtherActor))
  (`self.Fade Widget`)
  (bind _output_get (set `self.BP Pippa Character` _asbp_pippa_character))
  ;[0.01758 0.2458 0.3142] Modify Camera
  (`SceneComponent.K2_AttachToComponent` (`PippaCharacter.Camera` _output_get) (`PippaCharacter.SpringArm` _output_get) "None" "KeepRelative" "KeepRelative" "KeepRelative" true)
  ;[0.01198 0.09048 0.342] Send Pippa Back and Reset IMC
  (`self.K2_SetActorLocationAndRotation` :`self` (`self.BP Pippa Character`) :`NewLocation` (`SceneComponent.K2_GetComponentLocation` (`self.InLandingPlayerStart`)))
  (`EnhancedInputSubsystemInterface.RemoveMappingContext` (pcsubsystem `EnhancedInputLocalPlayerSubsystem` (`GameplayStatics.GetPlayerController` 0)) "/Game/Blueprints/Input/IMC_RotateRight_PippaContext.IMC_RotateRight_PippaContext" (struct)))

(event `Fade Widget`
  (bind _returnvalue (`FQFBlueprintFunctionLibrary.GetFQFGameMode` self))
  (bind _asbp_fqfgame_mode_base (cast `/Game/Blueprints/Game/BP_FQFGameModeBase` _returnvalue))
  (bind _newparam (`/Game/Blueprints/Game/BP_FQFGameModeBase.SpawnFadeWidget` _asbp_fqfgame_mode_base))
  (`KismetSystemLibrary.Delay` 0.5)
  (`Widget.RemoveFromParent` _newparam))

(fn `UserConstructionScript`)