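; Left-hand hotel door actor that tracks the player entering and leaving a room through its RoomCollision overlap volume.
; Entering sends DoorLocation to the player pawn's hotel state message and broadcasts EnteredNewRoom with that location.
; Leaving resends DoorLocation to the pawn but broadcasts Landing, then after a short delay asks the game mode to spawn a timed wave of slimes at the landing's point collection.
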(event `self.RoomCollision.OnComponentBeginOverlap`
  (params (OverlappedComponent :type "PrimitiveComponent Object Reference") (OtherActor :type "Actor Object Reference") (OtherComp :type "PrimitiveComponent Object Reference") (OtherBodyIndex :type Integer) (bFromSweep :type Boolean) (SweepResult :type "HitResult Structure (by ref)"))
  (bind _returnvalue (`GameplayStatics.GetPlayerPawn` 0))
  ;[0.5727 1 0.796] Overlaps
  (if (== OtherActor _returnvalue)
    (message `/Game/Blueprints/Interfaces/BPI_PlayerInterface.SetPippaHotelState` _returnvalue (`self.DoorLocation`))
    (`self.EnteredNewRoom` (`self.DoorLocation`))))

(event `self.RoomCollision.OnComponentEndOverlap`
  (params (OverlappedComponent :type "PrimitiveComponent Object Reference") (OtherActor :type "Actor Object Reference") (OtherComp :type "PrimitiveComponent Object Reference") (OtherBodyIndex :type Integer))
  (bind _returnvalue (`GameplayStatics.GetPlayerPawn` 0))
  ;[0.5727 1 0.796] Overlaps
  (if (== OtherActor _returnvalue)
    (message `/Game/Blueprints/Interfaces/BPI_PlayerInterface.SetPippaHotelState` _returnvalue (`self.DoorLocation`))
    (`self.EnteredNewRoom` "Landing")
    (`KismetSystemLibrary.Delay` 1.5)
    (bind _returnvalue_2 (`FQFBlueprintFunctionLibrary.GetFQFGameMode` (`GameplayStatics.GetPlayerPawn` 0)))
    (bind _asbp_fqfgame_mode_base (cast `/Game/Blueprints/Game/BP_FQFGameModeBase` _returnvalue_2))
    (`/Game/Blueprints/Game/BP_FQFGameModeBase.GenericSpawnSequence` _asbp_fqfgame_mode_base (make `/Game/Blueprints/Game/S_SpawnSequenceData` 6.0 0.2 0.0 "/Game/Blueprints/Character/Enemy/SlimeMonster/BP_SlimeL1.BP_SlimeL1_C" "/Game/Blueprints/Actor/SpawnPoints/Hotel/BP_HotelRoomLanding_PointCollection.BP_HotelRoomLanding_PointCollection_C" 1 null (0.0 0.0 0.0) "Landing"))))

(fn `UserConstructionScript`
  (`parent.UserConstructionScript`))