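; BP_LandingDoor is a door that switches camera and input context as an actor passes through, and starts the level on first entry.
; After a short delay, the enter trigger notifies PippaPlayerController once, while both triggers check the overlapping actor's facing.
; Enter attaches the camera to the Arrow point and exit returns it to the spring arm, via messages.
; OpenDoorSlowly swings the mesh's yaw with a left or right timeline.
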(event `self.Enter Door Collision.OnComponentBeginOverlap`
  (params (OverlappedComponent :type "PrimitiveComponent Object Reference") (OtherActor :type "Actor Object Reference") (OtherComp :type "PrimitiveComponent Object Reference") (OtherBodyIndex :type Integer) (bFromSweep :type Boolean) (SweepResult :type "HitResult Structure (by ref)"))
  ;[0.5727 1 0.796] Overlaps
  (set `self.OverlappedActor` OtherActor)
  (`KismetSystemLibrary.Delay` 0.2)
  (if (not (`self.AlreadyBeenThrough`))
    (set `self.AlreadyBeenThrough` true)
    (`self.NotifyShouldBeginLevel`))
  (bind _is_facing_default (message `/Game/Blueprints/Interfaces/BPI_PlayerInterface.IsPlayerFacingDefault` (`self.OverlappedActor`)))
  (if _is_facing_default
    (message `/Game/Blueprints/Interfaces/BPI_PlayerInterface.AttachCameraToPoint` (`self.OverlappedActor`) (`self.Arrow`) true)
    (message `/Game/Blueprints/Interfaces/BPI_PlayerInterface.ModifyMappingContext` (`self.OverlappedActor`) (`self.MappingContextRequired`))))

(event `self.Exit Door Collision.OnComponentBeginOverlap`
  (params (OverlappedComponent :type "PrimitiveComponent Object Reference") (OtherActor :type "Actor Object Reference") (OtherComp :type "PrimitiveComponent Object Reference") (OtherBodyIndex :type Integer) (bFromSweep :type Boolean) (SweepResult :type "HitResult Structure (by ref)"))
  ;[0.5727 1 0.796] Overlaps
  (set `self.OverlappedActor` OtherActor)
  (`KismetSystemLibrary.Delay` 0.2)
  (bind _is_facing_default (message `/Game/Blueprints/Interfaces/BPI_PlayerInterface.IsPlayerFacingDefault` (`self.OverlappedActor`)))
  (if (not _is_facing_default)
    (message `/Game/Blueprints/Interfaces/BPI_PlayerInterface.AttachCameraToSpringArm` (`self.OverlappedActor`))
    (message `/Game/Blueprints/Interfaces/BPI_PlayerInterface.ModifyMappingContext` (`self.OverlappedActor`) (`self.MappingContextRequired`))))

(event `OpenDoorSlowly`
  (params (`Is RHS` :type Boolean))
  (bind (_returnvalue_roll _returnvalue_pitch) (`KismetMathLibrary.BreakRotator` (`SceneComponent.K2_GetComponentRotation` (`self.SM_Door`))))
  (bind (_returnvalue_roll_2 _returnvalue_pitch_2) (`KismetMathLibrary.BreakRotator` (`SceneComponent.K2_GetComponentRotation` (`self.SM_Door`))))
  ;[0.3733 0.04056 0.169] Open Door Slowly
  (if `Is RHS`
    (bind (_direction _rhs_doorangle) (`Timeline|RHS Door opening`)
      (:`Update`
        (`SceneComponent.K2_SetWorldRotation` (`self.SM_Door`) (`KismetMathLibrary.MakeRotator` _returnvalue_roll _returnvalue_pitch _rhs_doorangle) false false)))
    (else
      (bind (_direction_2 _rhs_doorangle_2 _lhs_door_angle) (`Timeline|LHS Door Opening`)
        (:`Update`
          (`SceneComponent.K2_SetWorldRotation` (`self.SM_Door`) (`KismetMathLibrary.MakeRotator` _returnvalue_roll_2 _returnvalue_pitch_2 _lhs_door_angle) false false))))))

(fn `NotifyShouldBeginLevel`
  (bind _aspippa_player_controller (cast `PippaPlayerController` (`GameplayStatics.GetPlayerController` 0)))
  (set `PippaPlayerController.bLevelIsRunning` true _aspippa_player_controller)
  (`PippaPlayerController.BroadcastLevelShouldBegin` _aspippa_player_controller))

(fn `UserConstructionScript`)