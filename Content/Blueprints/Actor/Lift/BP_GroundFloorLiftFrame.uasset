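; BP_GroundFloorLiftFrame is the ground floor lift frame actor, which shows a countdown for the lift.
; BeginLiftCountdown stores the starting value and runs a looping one-second timer that decrements it and refreshes the display.
; A parallel Delay of the same length forces the display to zero and clears the timer.
; SetCountdownText writes the value into the WBP_LiftCountdown widget hosted by the frame's widget component.
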(event `self.ReceiveBeginPlay`)

(event `BeginLiftCountdown`
  (params (StartingValue :type "Float (double-precision)"))
  (bind _output_get (set `self.Time` StartingValue))
  (`self.Set Countdown Text` _output_get)
  (bind _returnvalue (`KismetSystemLibrary.K2_SetTimerDelegate` (delegate `Update Countdown Text`) 1.0 true))
  (`KismetSystemLibrary.Delay` StartingValue)
  (`self.Set Countdown Text` 0.0)
  (`KismetSystemLibrary.K2_ClearAndInvalidateTimerHandle` _returnvalue))

(event `Update Countdown Text`
  (bind _result (`/Engine/EditorBlueprintResources/StandardMacros.DecrementFloat` (`self.Time`))
    (:`  `
      (`self.Set Countdown Text` _result))))

(fn `Set Countdown Text`
  (params (Value :type "Float (double-precision)"))
  (bind _aswbp_lift_countdown (cast `/Game/Blueprints/UI/FloatingText/WBP_LiftCountdown` (`WidgetComponent.GetUserWidgetObject` (`self.BP_LiftCountdownTextComponent`))))
  (set `self.Countdown Text` (`/Game/Blueprints/UI/FloatingText/WBP_LiftCountdown.CountdownText` _aswbp_lift_countdown))
  (`TextBlock.SetText` (`self.Countdown Text`) (`KismetTextLibrary.Conv_DoubleToText` Value "HalfToEven" false true 1 324 0 0)))

(fn `UserConstructionScript`)