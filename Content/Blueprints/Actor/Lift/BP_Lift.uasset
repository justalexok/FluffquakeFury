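; Lift actor that shuttles endlessly between the ground floor and basement on a timed cycle started at BeginPlay.
; LiftCycle chains delays around door and move events, sending the total cycle time to the ground-floor frame's countdown each loop.
; Timelines slide the car's doors with the current floor frame's doors and interpolate the car's Z toward the other frame.
; Player overlap attaches the camera to CameraArrow; the logic clearing the inside flag is disconnected.
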(event `self.ReceiveTick`
  (params (DeltaSeconds :type "Float (single-precision)")))

(event `self.ReceiveBeginPlay`
  (`self.Calculate Total Cycle Time`)
  (set `self.Lift Position` "NewEnumerator0")
  (`self.Lift Cycle`))

(event `Lift Cycle`
  ;[0.7778 0.207 0.0139] Lift Cycle
  (`self.open lift doors` :!label _label)
  (`KismetSystemLibrary.Delay` (`self.Door Open Time`))
  (`KismetSystemLibrary.Delay` (`self.Lift Wait Time`))
  (`self.Close Lift Doors`)
  (`KismetSystemLibrary.Delay` (`self.Door Open Time`))
  (bind _returnvalue (`GameplayStatics.GetActorOfClass` "/Game/Blueprints/Actor/Lift/BP_GroundFloorLiftFrame.BP_GroundFloorLiftFrame_C"))
  (`/Game/Blueprints/Actor/Lift/BP_GroundFloorLiftFrame.BeginLiftCountdown` _returnvalue (`self.TotalCycleTime`))
  (`self.Move Lift`)
  (`KismetSystemLibrary.Delay` (`self.Lift Move Time`))
  (`self.open lift doors`)
  (`KismetSystemLibrary.Delay` (`self.Door Open Time`))
  (`KismetSystemLibrary.Delay` (`self.Lift Wait Time`))
  (`self.Close Lift Doors`)
  (`KismetSystemLibrary.Delay` (`self.Door Open Time`))
  (`self.Move Lift`)
  (`KismetSystemLibrary.Delay` (`self.Lift Move Time`))
  (goto _label))

(event `open lift doors`
  (bind (_left_lift_door_starting_location_x _left_lift_door_starting_location_y _left_lift_door_starting_location_z) (`KismetMathLibrary.BreakVector` (`self.Left Lift Door Starting Location`)))
  (bind (_left_ground_floor_door_starting_location_x _left_ground_floor_door_starting_location_y _left_ground_floor_door_starting_location_z) (`KismetMathLibrary.BreakVector` (`self.Left Ground Floor Door Starting Location`)))
  (bind (_left_basement_door_starting_location_x _left_basement_door_starting_location_y _left_basement_door_starting_location_z) (`KismetMathLibrary.BreakVector` (`self.Left Basement Door Starting Location`)))
  (bind (_right_basement_door_starting_location_x _right_basement_door_starting_location_y _right_basement_door_starting_location_z) (`KismetMathLibrary.BreakVector` (`self.Right Basement Door Starting Location`)))
  (bind (_right_lift_door_starting_locatin_x _right_lift_door_starting_locatin_y _right_lift_door_starting_locatin_z) (`KismetMathLibrary.BreakVector` (`self.Right Lift Door Starting Locatin`)))
  (bind (_right_ground_floor_door_starting_location_x _right_ground_floor_door_starting_location_y _right_ground_floor_door_starting_location_z) (`KismetMathLibrary.BreakVector` (`self.Right Ground Floor Door Starting Location`)))
  ;[0.02353 0.09804 0.04706] Open Doors
  (`self.Set Starting Locations`)
  (bind (_direction _door_y_position) (`Timeline|Door Y position Timeline` :!via `PlayFromStart`)
    (:`Update`
      (`SceneComponent.K2_SetWorldLocation` (`self.DoorLeft`) (`KismetMathLibrary.MakeVector` _left_lift_door_starting_location_x (+ _left_lift_door_starting_location_y _door_y_position) _left_lift_door_starting_location_z) false false)
      (`SceneComponent.K2_SetWorldLocation` (`self.DoorRight`) (`KismetMathLibrary.MakeVector` _right_lift_door_starting_locatin_x (- _right_lift_door_starting_locatin_y _door_y_position) _right_lift_door_starting_locatin_z) false false)
      (switch `/Game/Blueprints/Actor/Lift/E_LiftPosition` (`self.Lift Position`)
        (:`NewEnumerator0`
          ;;[1 1 1] Move Ground Floor
          (`SceneComponent.K2_SetWorldLocation` (`self.GroundFloor LeftDoor`) (`KismetMathLibrary.MakeVector` _left_ground_floor_door_starting_location_x (+ _left_ground_floor_door_starting_location_y _door_y_position) _left_ground_floor_door_starting_location_z) false false)
          (`SceneComponent.K2_SetWorldLocation` (`self.GroundFloor RightDoor`) (`KismetMathLibrary.MakeVector` _right_ground_floor_door_starting_location_x (- _right_ground_floor_door_starting_location_y _door_y_position) _right_ground_floor_door_starting_location_z) false false))
        (:`NewEnumerator1`
          ;;[1 1 1] Move Basement
          (`SceneComponent.K2_SetWorldLocation` (`self.Basement Left Door`) (`KismetMathLibrary.MakeVector` _left_basement_door_starting_location_x (+ _left_basement_door_starting_location_y _door_y_position) _left_basement_door_starting_location_z) false false)
          (`SceneComponent.K2_SetWorldLocation` (`self.Basement Right Door`) (`KismetMathLibrary.MakeVector` _right_basement_door_starting_location_x (- _right_basement_door_starting_location_y _door_y_position) _right_basement_door_starting_location_z) false false))))))

(event `Close Lift Doors`
  (bind (_right_ground_floor_door_starting_location_x _right_ground_floor_door_starting_location_y _right_ground_floor_door_starting_location_z) (`KismetMathLibrary.BreakVector` (`self.Right Ground Floor Door Starting Location`)))
  (bind (_right_lift_door_starting_locatin_x _right_lift_door_starting_locatin_y _right_lift_door_starting_locatin_z) (`KismetMathLibrary.BreakVector` (`self.Right Lift Door Starting Locatin`)))
  (bind (_left_ground_floor_door_starting_location_x _left_ground_floor_door_starting_location_y _left_ground_floor_door_starting_location_z) (`KismetMathLibrary.BreakVector` (`self.Left Ground Floor Door Starting Location`)))
  (bind (_left_lift_door_starting_location_x _left_lift_door_starting_location_y _left_lift_door_starting_location_z) (`KismetMathLibrary.BreakVector` (`self.Left Lift Door Starting Location`)))
  (bind (_left_basement_door_starting_location_x _left_basement_door_starting_location_y _left_basement_door_starting_location_z) (`KismetMathLibrary.BreakVector` (`self.Left Basement Door Starting Location`)))
  (bind (_right_basement_door_starting_location_x _right_basement_door_starting_location_y _right_basement_door_starting_location_z) (`KismetMathLibrary.BreakVector` (`self.Right Basement Door Starting Location`)))
  ;[0.02353 0.09804 0.04706] Close Doors
  (`self.Set Starting Locations`)
  (bind (_direction _door_opening_y_position) (`Timeline|Timeline` :!via `PlayFromStart`)
    (:`Update`
      (`SceneComponent.K2_SetWorldLocation` (`self.DoorLeft`) (`KismetMathLibrary.MakeVector` _left_lift_door_starting_location_x (- _left_lift_door_starting_location_y _door_opening_y_position) _left_lift_door_starting_location_z) false false)
      (`SceneComponent.K2_SetWorldLocation` (`self.DoorRight`) (`KismetMathLibrary.MakeVector` _right_lift_door_starting_locatin_x (+ _right_lift_door_starting_locatin_y _door_opening_y_position) _right_lift_door_starting_locatin_z) false false)
      (switch `/Game/Blueprints/Actor/Lift/E_LiftPosition` (`self.Lift Position`)
        (:`NewEnumerator0`
          ;;[1 1 1] Move Ground Floor
          (`SceneComponent.K2_SetWorldLocation` (`self.GroundFloor LeftDoor`) (`KismetMathLibrary.MakeVector` _left_ground_floor_door_starting_location_x (- _left_ground_floor_door_starting_location_y _door_opening_y_position) _left_ground_floor_door_starting_location_z) false false)
          (`SceneComponent.K2_SetWorldLocation` (`self.GroundFloor RightDoor`) (`KismetMathLibrary.MakeVector` _right_ground_floor_door_starting_location_x (+ _right_ground_floor_door_starting_location_y _door_opening_y_position) _right_ground_floor_door_starting_location_z) false false))
        (:`NewEnumerator1`
          ;;[1 1 1] Move Basement
          (`SceneComponent.K2_SetWorldLocation` (`self.Basement Left Door`) (`KismetMathLibrary.MakeVector` _left_basement_door_starting_location_x (- _left_basement_door_starting_location_y _door_opening_y_position) _left_basement_door_starting_location_z) false false)
          (`SceneComponent.K2_SetWorldLocation` (`self.Basement Right Door`) (`KismetMathLibrary.MakeVector` _right_basement_door_starting_location_x (+ _right_basement_door_starting_location_y _door_opening_y_position) _right_basement_door_starting_location_z) false false))))))

(event `self.InsideCollisionBox.OnComponentBeginOverlap`
  (params (OverlappedComponent :type "PrimitiveComponent Object Reference") (OtherActor :type "Actor Object Reference") (OtherComp :type "PrimitiveComponent Object Reference") (OtherBodyIndex :type Integer) (bFromSweep :type Boolean) (SweepResult :type "HitResult Structure (by ref)"))
  ;[0.6615 0 0.04132] Pippa enters or leaves lift
  (if (== OtherActor (`GameplayStatics.GetPlayerPawn` 0))
    (set `self.PippaIsInsideLift` true)
    (message `/Game/Blueprints/Interfaces/BPI_PlayerInterface.AttachCameraToPoint` (`GameplayStatics.GetPlayerPawn` 0) (`self.CameraArrow`) false)))

(event `self.InsideCollisionBox.OnComponentEndOverlap`
  (params (OverlappedComponent :type "PrimitiveComponent Object Reference") (OtherActor :type "Actor Object Reference") (OtherComp :type "PrimitiveComponent Object Reference") (OtherBodyIndex :type Integer))
  ;[0.6615 0 0.04132] Pippa enters or leaves lift
)

(event `Move Lift`
  (bind (_target_location_x _target_location_y _target_location_z) (`KismetMathLibrary.BreakVector` (`self.Target Location`)))
  (bind (_lift_starting_location_x _lift_starting_location_y _lift_starting_location_z) (`KismetMathLibrary.BreakVector` (`self.Lift Starting Location`)))
  (bind (_target_location_x_2 _target_location_y_2 _target_location_z_2) (`KismetMathLibrary.BreakVector` (`self.Target Location`)))
  (bind (_lift_starting_location_x_2 _lift_starting_location_y_2 _lift_starting_location_z_2) (`KismetMathLibrary.BreakVector` (`self.Lift Starting Location`)))
  ;[0.152 0.5955 0.2852] Move Lift
  (switch `/Game/Blueprints/Actor/Lift/E_LiftPosition` (`self.Lift Position`)
    (:`NewEnumerator0`
      (bind _returnvalue (`GameplayStatics.GetActorOfClass` "/Game/Blueprints/Actor/Lift/BP_0BasementLiftFrame.BP_0BasementLiftFrame_C"))
      (set `self.Target Location` (`SceneComponent.K2_GetComponentLocation` (`StaticMeshActor.StaticMeshComponent` _returnvalue)))
      (bind (_direction _normalizedliftz) (`Timeline|LiftDownTimeline` :!via `PlayFromStart`)
        (:`Update`
          (`self.K2_SetActorLocation` (`KismetMathLibrary.MakeVector` _lift_starting_location_x _lift_starting_location_y (+ _lift_starting_location_z (* (- _target_location_z _lift_starting_location_z) _normalizedliftz)))))
        (:`Finished`
          (set `self.Lift Position` "NewEnumerator1"))))
    (:`NewEnumerator1`
      (bind _returnvalue_2 (`GameplayStatics.GetActorOfClass` "/Game/Blueprints/Actor/Lift/BP_GroundFloorLiftFrame.BP_GroundFloorLiftFrame_C"))
      (set `self.Target Location` (`SceneComponent.K2_GetComponentLocation` (`StaticMeshActor.StaticMeshComponent` _returnvalue_2)))
      (bind (_direction_2 _normalizedliftz_2) (`Timeline|Timeline_0` :!via `PlayFromStart`)
        (:`Update`
          (`self.K2_SetActorLocation` (`KismetMathLibrary.MakeVector` _lift_starting_location_x_2 _lift_starting_location_y_2 (+ _lift_starting_location_z_2 (* (- _target_location_z_2 _lift_starting_location_z_2) _normalizedliftz_2)))))
        (:`Finished`
          (set `self.Lift Position` "NewEnumerator0"))))))

(fn `Calculate Total Cycle Time`
  (set `self.TotalCycleTime` (+ (* (`self.Lift Wait Time`) 2.0) (* (`self.Lift Move Time`) 2.0) (* (`self.Door Open Time`) 4.0))))

(fn `Set Starting Locations`
  (`|ExecutionSequence`
    (:`then_0`
      (set `self.Left Lift Door Starting Location` (`SceneComponent.K2_GetComponentLocation` (`self.DoorLeft`)))
      (set `self.Right Lift Door Starting Locatin` (`SceneComponent.K2_GetComponentLocation` (`self.DoorRight`)))
      (set `self.Lift Starting Location` (`self.K2_GetActorLocation`)))
    (:`then_1`
      (bind _outactors (`GameplayStatics.GetAllActorsOfClassWithTag` "/Game/Blueprints/Actor/Lift/BP_GroundFloorLiftFrame.BP_GroundFloorLiftFrame_C" "Ground"))
      (for _array_element _outactors
        (bind _leftdoor (`/Game/Blueprints/Actor/Lift/BP_GroundFloorLiftFrame.LeftDoor` _array_element))
        (set `self.GroundFloor LeftDoor` _leftdoor)
        (set `self.Left Ground Floor Door Starting Location` (`SceneComponent.K2_GetComponentLocation` _leftdoor))
        (bind _rightdoor (`/Game/Blueprints/Actor/Lift/BP_GroundFloorLiftFrame.RightDoor` _array_element))
        (set `self.Right Ground Floor Door Starting Location` (`SceneComponent.K2_GetComponentLocation` _rightdoor))
        (set `self.GroundFloor RightDoor` _rightdoor)))
    (:`then_2`
      (bind _returnvalue (`GameplayStatics.GetActorOfClass` "/Game/Blueprints/Actor/Lift/BP_0BasementLiftFrame.BP_0BasementLiftFrame_C"))
      (bind _output_get (set `self.Basement Left Door` (`/Game/Blueprints/Actor/Lift/BP_GroundFloorLiftFrame.LeftDoor` _returnvalue)))
      (set `self.Left Basement Door Starting Location` (`SceneComponent.K2_GetComponentLocation` _output_get))
      (bind _output_get_2 (set `self.Basement Right Door` (`/Game/Blueprints/Actor/Lift/BP_GroundFloorLiftFrame.RightDoor` _returnvalue)))
      (set `self.Right Basement Door Starting Location` (`SceneComponent.K2_GetComponentLocation` _output_get_2)))))

(fn `UserConstructionScript`)