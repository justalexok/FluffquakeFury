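; BP_ZoomOutCameraPoint is an actor marking a zoom-out camera viewpoint for a sliding glass door with a handle.
; SetZoomOutPointLocation places its root at a fixed world-space offset from the door handle, raised and using the door's rotation pitched downward.
; An unconnected EventGraph chain would find the regular door, falling back to the small variant, but BeginPlay is empty, so the actor never repositions itself.
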(event `self.ReceiveBeginPlay`)

(fn `Set Zoom Out Point Location`
  (params (SlidingDoor :type "/Game/Blueprints/Actor/GlassDoors/BP_SlidingGlassDoorWithHandle Object Reference"))
  (`SceneComponent.K2_SetWorldLocationAndRotation` (`self.DefaultSceneRoot`) (- (`SceneComponent.K2_GetComponentLocation` (`/Game/Blueprints/Actor/GlassDoors/BP_SlidingGlassDoorWithHandle.DoorHandle` SlidingDoor)) (325.0 0.0 -100.0)) (`KismetMathLibrary.MakeRotator` (.roll (`self.K2_GetActorRotation` SlidingDoor)) (- (.pitch (`self.K2_GetActorRotation` SlidingDoor)) 25.0) (.yaw (`self.K2_GetActorRotation` SlidingDoor))) false false))

(fn `UserConstructionScript`)