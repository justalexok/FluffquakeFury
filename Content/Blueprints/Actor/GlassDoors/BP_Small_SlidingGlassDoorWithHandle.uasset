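; Small sliding glass door with handle, a child Blueprint that overrides its parent's MoveDoors function without calling the parent version.
; MoveDoors slides the left and right meshes apart at constant speed using VInterpToConstant toward fixed offsets from their stored world locations.
; The offsets lie on the world Y axis, so the slide direction ignores actor rotation.
; The event graph is inactive and the construction script only calls the parent.
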(fn `MoveDoors`
  (params (DeltaTime :type "Float (single-precision)"))
  (`SceneComponent.K2_SetWorldLocation` (`self.LeftDoorMesh`) (`KismetMathLibrary.VInterpTo_Constant` (`SceneComponent.K2_GetComponentLocation` (`self.LeftDoorMesh`)) (+ (`self.LeftDoorWorldLocation`) (0.0 -100.0 0.0)) (`local.DeltaTime`) 50.0) false false)
  (`SceneComponent.K2_SetWorldLocation` (`self.RightDoorMesh`) (`KismetMathLibrary.VInterpTo_Constant` (`SceneComponent.K2_GetComponentLocation` (`self.RightDoorMesh`)) (+ (`self.RightDoorWorldLocation`) (0.0 100.0 0.0)) (`local.DeltaTime`) 50.0) false false))

(fn `UserConstructionScript`
  (`parent.UserConstructionScript`))