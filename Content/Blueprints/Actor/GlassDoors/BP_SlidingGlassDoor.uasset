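; Sliding glass door actor that runs a scripted sequence with the player (Pippa), opening with sound, smoke and a camera zoom-out.
; Player overlap disables input and sends the pawn a MovePippa message.
; ShouldOpenDoors waits briefly, then opens the doors, fires effects and attaches the camera to BP_ZoomOutCameraPoint.
; Timelines slide both meshes along world Y from BeginPlay positions; the level-fade chain and MoveDoorsDep are unused.
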(event `self.ReceiveBeginPlay`
  (set `self.LeftDoorWorldLocation` (`SceneComponent.K2_GetComponentLocation` (`self.LeftDoorMesh`)))
  (set `self.RightDoorWorldLocation` (`SceneComponent.K2_GetComponentLocation` (`self.RightDoorMesh`)))
  (bind _asbp_fqfgame_mode_base (cast `/Game/Blueprints/Game/BP_FQFGameModeBase` (`GameplayStatics.GetGameMode`)))
  (set `self.FQFGame Mode` _asbp_fqfgame_mode_base))

(event `self.ReceiveTick`
  (params (DeltaSeconds :type "Float (single-precision)")))

(event `self.CollisionBox.OnComponentBeginOverlap`
  (params (OverlappedComponent :type "PrimitiveComponent Object Reference") (OtherActor :type "Actor Object Reference") (OtherComp :type "PrimitiveComponent Object Reference") (OtherBodyIndex :type Integer) (bFromSweep :type Boolean) (SweepResult :type "HitResult Structure (by ref)"))
  (bind _returnvalue (`GameplayStatics.GetPlayerPawn` 0))
  (if (== OtherActor _returnvalue)
    (`PrimitiveComponent.SetCollisionResponseToChannel` (`self.CollisionBox`) "ECC_WorldStatic" "ECR_Ignore")
    (`self.DisableInput` (`GameplayStatics.GetPlayerController` 0) null)
    (message `/Game/Blueprints/Interfaces/BPI_PlayerInterface.MovePippa` _returnvalue)))

(event `ShouldOpenDoors`
  (`KismetSystemLibrary.Delay` 1.0)
  (`self.OpenDoors`)
  (`GameplayStatics.PlaySoundAtLocation` "/Game/AGContent/SFX/Misc/SlidingDoors.SlidingDoors" (`SceneComponent.K2_GetComponentLocation` (`self.CentralGroundPoint`)) (struct) 1.0 1.0 0.0 null null null null)
  (`ActorComponent.Activate` (`self.SmokeNiagara`) false)
  (bind _returnvalue (`GameplayStatics.GetActorOfClass` "/Game/Blueprints/Actor/GlassDoors/BP_ZoomOutCameraPoint.BP_ZoomOutCameraPoint_C"))
  (message `/Game/Blueprints/Interfaces/BPI_PlayerInterface.AttachCameraToPoint` (`GameplayStatics.GetPlayerPawn` 0) (`/Game/Blueprints/Actor/GlassDoors/BP_ZoomOutCameraPoint.Arrow` _returnvalue) false))

(event `OpenDoors`
  (bind (_leftdoorworldlocation_x _leftdoorworldlocation_y _leftdoorworldlocation_z) (`KismetMathLibrary.BreakVector` (`self.LeftDoorWorldLocation`)))
  (bind (_rightdoorworldlocation_x _rightdoorworldlocation_y _rightdoorworldlocation_z) (`KismetMathLibrary.BreakVector` (`self.RightDoorWorldLocation`)))
  ;[1 0.6256 0.7438] Open Doors
  (bind (_direction _door_y_position) (`Timeline|Open Doors`)
    (:`Update`
      (`SceneComponent.K2_SetWorldLocation` (`self.LeftDoorMesh`) (`KismetMathLibrary.MakeVector` _leftdoorworldlocation_x (+ _leftdoorworldlocation_y (* _door_y_position -1.0)) _leftdoorworldlocation_z) false false)
      (`SceneComponent.K2_SetWorldLocation` (`self.RightDoorMesh`) (`KismetMathLibrary.MakeVector` _rightdoorworldlocation_x (+ _rightdoorworldlocation_y _door_y_position) _rightdoorworldlocation_z) false false))))

(event `CloseDoors`
  (bind (_leftdoorworldlocation_x _leftdoorworldlocation_y _leftdoorworldlocation_z) (`KismetMathLibrary.BreakVector` (`self.LeftDoorWorldLocation`)))
  (bind (_rightdoorworldlocation_x _rightdoorworldlocation_y _rightdoorworldlocation_z) (`KismetMathLibrary.BreakVector` (`self.RightDoorWorldLocation`)))
  ;[1 0.6256 0.7438] Close  Doors
  (bind (_direction _door_y_position) (`Timeline|Timeline`)
    (:`Update`
      (`SceneComponent.K2_SetWorldLocation` (`self.LeftDoorMesh`) (`KismetMathLibrary.MakeVector` _leftdoorworldlocation_x (+ _leftdoorworldlocation_y _door_y_position) _leftdoorworldlocation_z) false false)
      (`SceneComponent.K2_SetWorldLocation` (`self.RightDoorMesh`) (`KismetMathLibrary.MakeVector` _rightdoorworldlocation_x (+ _rightdoorworldlocation_y (* _door_y_position -1.0)) _rightdoorworldlocation_z) false false))))

(fn `Jolleen Begin Push`)

(fn `MoveDoors_dep`
  (params (DeltaTime :type "Float (single-precision)"))
  (locals (NewLocalVar :type "Float (single-precision)"))
  (`SceneComponent.K2_SetWorldLocation` (`self.LeftDoorMesh`) (`KismetMathLibrary.VInterpTo_Constant` (`SceneComponent.K2_GetComponentLocation` (`self.LeftDoorMesh`)) (+ (`self.LeftDoorWorldLocation`) (0.0 -150.0 0.0)) (`local.DeltaTime`) 50.0) false false)
  (`SceneComponent.K2_SetWorldLocation` (`self.RightDoorMesh`) (`KismetMathLibrary.VInterpTo_Constant` (`SceneComponent.K2_GetComponentLocation` (`self.RightDoorMesh`)) (+ (`self.RightDoorWorldLocation`) (0.0 150.0 0.0)) (`local.DeltaTime`) 50.0) false false))

(fn `Spawn FadeWidget`
  (bind _returnvalue (`|CreateWidget` "/Game/Blueprints/UI/Overlay/LevelWidgets/WBP_LevelFade.WBP_LevelFade_C"))
  (bind _output_get (set `self.FadeWidget` _returnvalue))
  (`UserWidget.AddToViewport` _output_get 0)
  (`/Game/Blueprints/UI/Overlay/LevelWidgets/WBP_LevelFade.PlayFadeAnim` (`self.FadeWidget`)))

(fn `UserConstructionScript`)