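; BP_SlidingGlassDoorWithHandle is a level-exit sliding glass door that opens on level completion and sends the player to the next streaming level.
; OpenDoors waits briefly, plays sound and smoke, moves Pippa's camera, and lets Tick slide both panels apart along world Y at constant speed.
; Any CollisionBox overlap runs a fade widget, calls the game mode's GoToNextStreamingLevel, disables the box and snaps the doors back to their cached positions.
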(event `self.ReceiveBeginPlay`
  (set `self.LeftDoorWorldLocation` (`SceneComponent.K2_GetComponentLocation` (`self.LeftDoorMesh`)))
  (set `self.RightDoorWorldLocation` (`SceneComponent.K2_GetComponentLocation` (`self.RightDoorMesh`)))
  (bind _asbp_fqfgame_mode_base (cast `/Game/Blueprints/Game/BP_FQFGameModeBase` (`GameplayStatics.GetGameMode`)))
  (set `self.FQFGame Mode` _asbp_fqfgame_mode_base))

(event `self.ReceiveTick`
  (params (DeltaSeconds :type "Float (single-precision)"))
  (if (`self.ShouldOpenDoors`)
    (`self.MoveDoors` DeltaSeconds)))

(event `self.CollisionBox.OnComponentBeginOverlap`
  (params (OverlappedComponent :type "PrimitiveComponent Object Reference") (OtherActor :type "Actor Object Reference") (OtherComp :type "PrimitiveComponent Object Reference") (OtherBodyIndex :type Integer) (bFromSweep :type Boolean) (SweepResult :type "HitResult Structure (by ref)"))
  ;[1 1 1] Level Complete - Go To Next Level
  (`KismetSystemLibrary.Delay` 0.25)
  (`self.Spawn FadeWidget`)
  (`KismetSystemLibrary.Delay` 0.5)
  (`Widget.RemoveFromParent` (`self.FadeWidget`))
  (`ActorComponent.Deactivate` (`self.SmokeNiagara`))
  (`/Game/Blueprints/Game/BP_FQFGameModeBase.Go To Next Streaming Level` (`self.FQFGame Mode`))
  (`PrimitiveComponent.SetCollisionEnabled` (`self.CollisionBox`) "NoCollision")
  (`self.SnapCloseDoors`))

(event `OpenDoors`
  (`KismetSystemLibrary.Delay` 1.0)
  (set `self.ShouldOpenDoors` true)
  (`GameplayStatics.PlaySoundAtLocation` "/Game/AGContent/SFX/SlidingDoors.SlidingDoors" (`SceneComponent.K2_GetComponentLocation` (`self.CentralGroundPoint`)) (struct) 1.0 1.0 0.0 null null null null)
  (`ActorComponent.Activate` (`self.SmokeNiagara`) false)
  (bind _asbp_pippa_character (cast `/Game/Blueprints/Character/Pippa/BP_PippaCharacter` (`GameplayStatics.GetPlayerPawn` 0)))
  (`/Game/Blueprints/Character/Pippa/BP_PippaCharacter.MoveCameraOnLevelCompletion` _asbp_pippa_character))

(event `SnapCloseDoors`
  (set `self.ShouldOpenDoors` false)
  (`SceneComponent.K2_SetWorldLocation` (`self.LeftDoorMesh`) (`self.LeftDoorWorldLocation`) false false)
  (`SceneComponent.K2_SetWorldLocation` (`self.RightDoorMesh`) (`self.RightDoorWorldLocation`) false false))

(fn `MoveDoors`
  (params (DeltaTime :type "Float (single-precision)"))
  (locals (NewLocalVar :type "Float (single-precision)"))
  (`SceneComponent.K2_SetWorldLocation` (`self.LeftDoorMesh`) (`KismetMathLibrary.VInterpTo_Constant` (`SceneComponent.K2_GetComponentLocation` (`self.LeftDoorMesh`)) (+ (`self.LeftDoorWorldLocation`) (0.0 -150.0 0.0)) (`local.DeltaTime`) 50.0) false false)
  (`SceneComponent.K2_SetWorldLocation` (`self.RightDoorMesh`) (`KismetMathLibrary.VInterpTo_Constant` (`SceneComponent.K2_GetComponentLocation` (`self.RightDoorMesh`)) (+ (`self.RightDoorWorldLocation`) (0.0 150.0 0.0)) (`local.DeltaTime`) 50.0) false false))

(fn `Spawn FadeWidget`
  (bind _returnvalue (`|CreateWidget` "/Game/Blueprints/UI/LevelWidgets/WBP_LevelFade.WBP_LevelFade_C"))
  (bind _output_get (set `self.FadeWidget` _returnvalue))
  (`UserWidget.AddToViewport` _output_get 0)
  (`/Game/Blueprints/UI/LevelWidgets/WBP_LevelFade.PlayFadeAnim` (`self.FadeWidget`)))

(fn `UserConstructionScript`)