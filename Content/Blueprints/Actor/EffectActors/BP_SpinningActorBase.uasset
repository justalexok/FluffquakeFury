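; Base actor for Jolleen's spinning attack, in which a thrown object such as a book hovers over Pippa, then drops on her.
; SpinAndDrop starts it with a waterball Niagara effect (skipped in HotelDemo), and Tick drives three flag-based phases: interpolate above Pippa, orbit that point, then home in.
; After SpinTime and a short delay, it sets collision to overlap, flags itself for destruction and clears Jolleen's casting state.
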(event `SpinAndDrop`
  (params (Caster :type "Actor Object Reference"))
  ;[0.003386 0.05314 0.1545] Set Variables
  (bind _asbp_jolleen (cast `/Game/Blueprints/Character/Enemy/Jolleen/BP_Jolleen` Caster))
  (set `self.BP Jolleen` _asbp_jolleen)
  (bind _asbp_pippa_character (cast `/Game/Blueprints/Character/Pippa/BP_PippaCharacter` (`Controller.K2_GetPawn` (`GameplayStatics.GetPlayerController` 0))))
  (set `self.BP Pippa Character` _asbp_pippa_character)
  (set `self.AttackHasBegun` true)
  (set `self.BooksTravelling` true)
  (set `self.SpinningSpeed` 1200.0)
  (`self.K2_SetActorRotation` (`KismetMathLibrary.MakeRotator` (`KismetMathLibrary.RandomFloatInRange` 0.0 180.0)))
  (`self.SpawnWaterBallNiagara`)
  ;[0.07401 0.007855 0.1545] Spin And Drop
  (`KismetSystemLibrary.Delay` (`self.SpinTime`))
  (set `self.BeginDrop` true)
  (bind _niagarasystem (`self.NiagaraSystem`)
    (:`then`
      (`ActorComponent.K2_DestroyComponent` _niagarasystem))
    (:`else`
      _))
  (`KismetSystemLibrary.Delay` 0.5)
  (`self.HandleEndOfSpinning`))

(event `self.ReceiveTick`
  (params (DeltaSeconds :type "Float (single-precision)"))
  (bind _output_get (set `self.Delta Seconds` DeltaSeconds))
  (`parent.ReceiveTick` _output_get)
  (if (`self.AttackHasBegun`)
    (if (`self.BooksTravelling`)
      ;[0.2279 0.02149 1] Books Travel
      (`self.SendBooksToTarget`)
      (`self.NotifyThatTargetIsInBounds`)
      (elif (`self.BeginDrop`)
        ;[0.2279 0.02149 1] Books Attack
        (`self.BooksHomeInOnTarget`)
        (else
          ;[0.2279 0.02149 1] Books Spin
          (`self.UpdateTargetLocation`)
          (`self.Set Current Rotation`)
          (`self.RotateActorAroundPoint` (`self.BookTargetLocation`) (`self.Radius`) (`self.StartingAngle`) (`self.CurrentRotation`)))))))

(fn `BooksHomeInOnTarget`
  (`self.K2_SetActorLocation` (`KismetMathLibrary.VInterpTo` (`self.K2_GetActorLocation`) (`self.K2_GetActorLocation` (`self.BP Pippa Character`)) (`self.Delta Seconds`) 10.0)))

(fn `HandleEndOfSpinning`
  (bind _bp_jolleen (`self.BP Jolleen`))
  (set `self.SpinningSpeed` 0.0)
  (set `self.ShouldBeDestroyed` true)
  (`PrimitiveComponent.SetCollisionResponseToChannel` (`self.CollisionBox`) "ECC_GameTraceChannel2" "ECR_Overlap")
  (`/Engine/EditorBlueprintResources/StandardMacros.IsValid` _bp_jolleen
    (:`Is Valid`
      (bind _returnvalue (message `CombatInterface.GetAnimInstance` _bp_jolleen))
      (bind _asabp_jolleen (cast `/Game/Blueprints/Character/Enemy/Jolleen/ABP_Jolleen` _returnvalue))
      (set `/Game/Blueprints/Character/Enemy/Jolleen/ABP_Jolleen.IsCasting` false _asabp_jolleen)
      (message `CombatInterface.SetBlackboardBoolForKey` (`self.BP Jolleen`) "AmICasting" false))))

(fn `NotifyThatTargetIsInBounds`
  (if (== (`self.BookTargetLocation`) (`self.BookCurrentLocation`) :`ErrorTolerance` (`self.AcceptanceRange`))
    (set `self.BooksTravelling` false)))

(fn `RotateActorAroundPoint`
  (params (TargetLocation :type "Vector Structure") (Radius :type "Float (double-precision)") (Angle :type "Float (double-precision)") (RotationRate :type "Float (double-precision)"))
  (locals (LActorToRotate :type "Actor Object Reference") (LTargetActor :type "Actor Object Reference") (LLocation :type "Vector Structure") (LRadius :type "Float (double-precision)") (LAngle :type "Float (double-precision)") (LRotationRate :type "Float (double-precision)"))
  (set `local.LTargetActor` null)
  (set `local.LLocation` TargetLocation)
  (set `local.LRadius` Radius)
  (set `local.LAngle` Angle)
  (set `local.LRotationRate` RotationRate)
  (`self.K2_SetActorLocation` (+ (`local.LLocation`) (`KismetMathLibrary.RotateAngleAxis` (`KismetMathLibrary.MakeVector` (`local.LRadius`)) (+ (`local.LAngle`) (`local.LRotationRate`)) (0.0 0.0 1.0))))
  (return))

(fn `SendBooksToTarget`
  (`self.UpdateTargetLocation`)
  (bind _output_get (set `self.BookCurrentLocation` (`self.K2_GetActorLocation`)))
  (`self.K2_SetActorLocation` (`KismetMathLibrary.VInterpTo` _output_get (`self.BookTargetLocation`) (`self.Delta Seconds`) (`self.Interp Speed`))))

(fn `Set Current Rotation`
  (set `self.CurrentRotation` (+ (`self.CurrentRotation`) (* (* (`self.RotationSpeed`) (`self.Delta Seconds`)) (`KismetMathLibrary.SelectFloat` 1.0 -1.0 (`self.Clockwise`))))))

(fn `SpawnWaterBallNiagara`
  (bind _returnvalue (`GameplayStatics.GetCurrentLevelName` true))
  (if (not (`KismetStringLibrary.MatchesWildcard` _returnvalue "HotelDemo"))
    (bind _returnvalue_2 (`NiagaraFunctionLibrary.SpawnSystemAttached` "/Game/AGContent/Niagara/FXVarietyPack/Particles/NS_Waterball.NS_Waterball" (`self.RootStaticMesh`) "None" (0.0 0.0 0.0) (struct) "KeepRelativeOffset"))
    (set `self.NiagaraSystem` _returnvalue_2)))

(fn `UpdateTargetLocation`
  (set `self.BookTargetLocation` (+ (`self.K2_GetActorLocation` (`self.BP Pippa Character`)) (`KismetMathLibrary.MakeVector` 0.0 0.0 (`self.Distance Above`)))))

(fn `UserConstructionScript`
  (`parent.UserConstructionScript`))