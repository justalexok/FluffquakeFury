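; Base pickup-style actor that spins in place and applies an instant Gameplay Effect to an actor that overlaps it.
; Tick drives the spin through RotateActor, while the CollisionBox overlap calls ApplyEffectToTarget with InstantGameplayEffectClass.
; On success it hides the root mesh, disables its collision responses, removes its child components and the box, then destroys itself after a short delay.
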(event `self.ReceiveTick`
  (params (DeltaSeconds :type "Float (single-precision)"))
  (`self.RotateActor` DeltaSeconds (`self.SpinningSpeed`)))

(event `self.CollisionBox.OnComponentBeginOverlap`
  (params (OverlappedComponent :type "PrimitiveComponent Object Reference") (OtherActor :type "Actor Object Reference") (OtherComp :type "PrimitiveComponent Object Reference") (OtherBodyIndex :type Integer) (bFromSweep :type Boolean) (SweepResult :type "HitResult Structure (by ref)"))
  (bind _output_get (set `self.OverlappedActor` OtherActor))
  (bind _returnvalue (`self.ApplyEffectToTarget` _output_get (`self.InstantGameplayEffectClass`)))
  (if _returnvalue
    (`self.HideAndDestroy`)))

(event `HideAndDestroy`
  (bind _rootstaticmesh (`self.RootStaticMesh`))
  (`SceneComponent.SetVisibility` _rootstaticmesh false true)
  (`PrimitiveComponent.SetCollisionResponseToAllChannels` _rootstaticmesh "ECR_Ignore")
  (for _array_element (`SceneComponent.GetChildrenComponents` _rootstaticmesh false)
    (`ActorComponent.K2_DestroyComponent` _array_element))
  (`ActorComponent.K2_DestroyComponent` (`self.CollisionBox`))
  (`KismetSystemLibrary.Delay` 0.7)
  (`self.K2_DestroyActor`))

(fn `UserConstructionScript`)