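; BP_Mirror is a mirror effect actor that is knocked over once when the player enters its trigger box.
; An overlap by a "Player"-tagged actor snaps the actor to a fixed rotation, then turns on physics for the root mesh and applies a velocity-change impulse.
; The trigger box then destroys itself so the effect cannot repeat.
; A debug "Triggered!" message prints on any overlap, before the tag check.
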(event `self.TriggerBox.OnComponentBeginOverlap`
  (params (OverlappedComponent :type "PrimitiveComponent Object Reference") (OtherActor :type "Actor Object Reference") (OtherComp :type "PrimitiveComponent Object Reference") (OtherBodyIndex :type Integer) (bFromSweep :type Boolean) (SweepResult :type "HitResult Structure (by ref)"))
  (`KismetSystemLibrary.PrintString` "Triggered!")
  (if (`self.ActorHasTag` OtherActor "Player")
    (bind _returnvalue (`self.K2_SetActorRotation` (struct :`Pitch` 45.0 :`Yaw` -90.0)))
    (if _returnvalue
      (`PrimitiveComponent.SetSimulatePhysics` (`self.RootStaticMesh`) true)
      (`PrimitiveComponent.AddImpulse` (`self.RootStaticMesh`) (0.0 100.0 20.0) "None" true)
      (bind _triggerbox (`self.TriggerBox`)
        (:`then`
          (`ActorComponent.K2_DestroyComponent` _triggerbox))
        (:`else`)))))

(fn `UserConstructionScript`
  (`parent.UserConstructionScript`))