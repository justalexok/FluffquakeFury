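; BP_PoisonPillow is a pickup actor that spins in place and adds one poison fluff to the player.
; Tick calls SpinPillow, which applies a constant yaw rotation scaled by delta time.
; When the player pawn overlaps the CollisionSphere, the pillow sends ModifyPoisonFluffCountMessage to that pawn to raise its count, then destroys itself.
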(event `self.ReceiveTick`
  (params (DeltaSeconds :type "Float (single-precision)"))
  (`self.SpinPillow` DeltaSeconds))

(event `self.CollisionSphere.OnComponentBeginOverlap`
  (params (OverlappedComponent :type "PrimitiveComponent Object Reference") (OtherActor :type "Actor Object Reference") (OtherComp :type "PrimitiveComponent Object Reference") (OtherBodyIndex :type Integer) (bFromSweep :type Boolean) (SweepResult :type "HitResult Structure (by ref)"))
  (bind _returnvalue (`GameplayStatics.GetPlayerPawn` 0))
  (if (== OtherActor _returnvalue)
    (message `/Game/Blueprints/Interfaces/BPI_PlayerInterface.ModifyPoisonFluffCount` _returnvalue 1)
    (`self.K2_DestroyActor`)))

(fn `SpinPillow`
  (params (`Delta Seconds` :type "Float (double-precision)"))
  (`self.K2_SetActorRotation` (`KismetMathLibrary.ComposeRotators` (`self.K2_GetActorRotation`) (`KismetMathLibrary.MakeRotator` 0.0 0.0 (* `Delta Seconds` 100.0)))))

(fn `UserConstructionScript`)