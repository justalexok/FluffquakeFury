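; Poison fog hazard that, on release, slows the player, flags Pippa's animation as stunned, shakes the camera and plays gas and coughing audio.
; A timeline animates fog extinction through a dynamic material instance and sets how long the poison stays active.
; FQF characters entering the active fog receive an infinite GAS poison effect, removed on exit or when the timeline finishes.
; Finishing also stops audio and shakes and restores the player.
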(event `self.ReceiveBeginPlay`
  (`PrimitiveComponent.SetCollisionEnabled` (`self.FogAreaCollision`) "NoCollision")
  (add `self.OnShouldReleasePoison` (delegate `OnShouldReleasePoison_Event`)))

(event `OnShouldReleasePoison_Event`
  ;[0.04224 1 0.1665] On Poison Released
  (set `self.IsActive` true)
  (`PrimitiveComponent.SetCollisionEnabled` (`self.FogAreaCollision`) "QueryOnly")
  (`self.Play Audio`)
  (message `CombatInterface.SetMaxWalkSpeedByFloat` (`GameplayStatics.GetPlayerPawn` 0) 92.0)
  (`self.SetPippaStunned` true)
  (`self.ShakeCamera`)
  (bind _returnvalue (`KismetMaterialLibrary.CreateDynamicMaterialInstance` (`self.GreenFogMaterialInstance`)))
  (`PrimitiveComponent.SetMaterial` (`self.FogArea`) 0 _returnvalue)
  (bind (_direction _normalized_fog_extinction) (`Timeline|Timeline` :!via `PlayFromStart`)
    (:`Update`
      (`MaterialInstanceDynamic.SetScalarParameterValue` _returnvalue "Extinction" _normalized_fog_extinction))
    (:`Finished`
      (set `self.IsActive` false)
      (`self.Poison Finished`))))

(event `Poison Finished`
  ;[0.000872 0.03646 0.01156] Poison Finished
  (`self.Stop Audio`)
  (`self.Handle Poison End for Pippa`)
  (for _array_element (`self.Poisoned Actors`)
    (`self.RemoveEffectFromTarget` _array_element)
    (`PrimitiveComponent.SetCollisionEnabled` (`self.FogAreaCollision`) "NoCollision"))
  (`KismetArrayLibrary.Array_Clear` (`self.Poisoned Actors`)))

(event `self.FogAreaCollision.OnComponentBeginOverlap`
  (params (OverlappedComponent :type "PrimitiveComponent Object Reference") (OtherActor :type "Actor Object Reference") (OtherComp :type "PrimitiveComponent Object Reference") (OtherBodyIndex :type Integer) (bFromSweep :type Boolean) (SweepResult :type "HitResult Structure (by ref)"))
  ;[0.5271 0.07227 0.05448] Overlap Events
  (bind _asfqfcharacter_base (cast `FQFCharacterBase` OtherActor))
  (if (`self.IsActive`)
    (`self.ApplyEffectToTarget` _asfqfcharacter_base)
    (`KismetArrayLibrary.Array_Add` (`self.Poisoned Actors`) _asfqfcharacter_base)))

(event `self.FogAreaCollision.OnComponentEndOverlap`
  (params (OverlappedComponent :type "PrimitiveComponent Object Reference") (OtherActor :type "Actor Object Reference") (OtherComp :type "PrimitiveComponent Object Reference") (OtherBodyIndex :type Integer))
  ;[0.5271 0.07227 0.05448] Overlap Events
  (bind _asfqfcharacter_base (cast `FQFCharacterBase` OtherActor))
  (`self.RemoveEffectFromTarget` _asfqfcharacter_base))

(fn `ApplyEffectToTarget`
  (params (TargetActor :type "FQFCharacterBase Object Reference"))
  (locals (ASC :type "AbilitySystemComponent Object Reference"))
  (bind _output_get (set `local.ASC` (`AbilitySystemBlueprintLibrary.GetAbilitySystemComponent` TargetActor)))
  (bind _returnvalue (`AbilitySystemComponent.BP_ApplyGameplayEffectSpecToSelf` (`local.ASC`) (`AbilitySystemComponent.MakeOutgoingSpec` (`local.ASC`) (`self.Infinite Poison Effect Class`) 1.0 (`AbilitySystemComponent.MakeEffectContext` _output_get))))
  (`BlueprintMapLibrary.Map_Add` (`FQFCharacterBase.ActiveInfiniteEffectHandles` TargetActor) _returnvalue (`local.ASC`)))

(fn `Handle Poison End for Pippa`
  (`PlayerCameraManager.StopAllCameraShakes` (`GameplayStatics.GetPlayerCameraManager` 0) true)
  (message `CombatInterface.SetMaxWalkSpeedByFloat` (`GameplayStatics.GetPlayerPawn` 0) 250.0)
  (`self.SetPippaStunned` false))

(fn `Play Audio`
  (`AudioComponent.Play` (`self.HissingGasAudio`) 0.0)
  (`AudioComponent.Play` (`self.CoughingAudio`) 0.0))

(fn `RemoveEffectFromTarget`
  (params (TargetActor :type "FQFCharacterBase Object Reference"))
  (locals (`Target Actor` :type "FQFCharacterBase Object Reference"))
  (`/Engine/EditorBlueprintResources/StandardMacros.IsValid` TargetActor
    (:`Is Valid`
      (bind _output_get (set `local.Target Actor` TargetActor))
      (bind _activeinfiniteeffecthandles (`FQFCharacterBase.ActiveInfiniteEffectHandles` _output_get))
      (bind _values (`BlueprintMapLibrary.Map_Values` _activeinfiniteeffecthandles))
      (for _array_element _values
        (bind _keys (`BlueprintMapLibrary.Map_Keys` _activeinfiniteeffecthandles))
        (for _array_element_2 _keys
          (`AbilitySystemComponent.RemoveActiveGameplayEffect` _array_element _array_element_2 -1))
        (`BlueprintMapLibrary.Map_Clear` (`FQFCharacterBase.ActiveInfiniteEffectHandles` (`local.Target Actor`)))))))

(fn `ScaleFogArea`
  (params (X :type "Float (double-precision)") (Y :type "Float (double-precision)") (Z :type "Float (double-precision)"))
  (bind (_targetscale_x _targetscale_y _targetscale_z) (`KismetMathLibrary.BreakVector` (`self.TargetScale`)))
  (bind _targetscale_x_2 (`KismetMathLibrary.BreakVector` (`self.TargetScale`)))
  (bind (_targetscale_x_3 _targetscale_y_2) (`KismetMathLibrary.BreakVector` (`self.TargetScale`)))
  (`SceneComponent.SetWorldScale3D` (`self.FogArea`) (`KismetMathLibrary.MakeVector` (* Z _targetscale_x_2) (* X _targetscale_y_2) (* _targetscale_z Y))))

(fn `SetPippaStunned`
  (params (`Is Stunned` :type Boolean))
  (bind _returnvalue (message `CombatInterface.GetAnimInstance` (`GameplayStatics.GetPlayerPawn` 0)))
  (bind _asabp_pippa_character (cast `/Game/Blueprints/Character/Pippa/ABP_PippaCharacter` _returnvalue))
  (set `/Game/Blueprints/Character/Pippa/ABP_PippaCharacter.IsStunned` `Is Stunned` _asabp_pippa_character))

(fn `ShakeCamera`
  (`GameplayStatics.PlayWorldCameraShake` "/Game/Blueprints/Game/CameraShakes/BP_InfiniteShake.BP_InfiniteShake_C" (`self.K2_GetActorLocation` (`GameplayStatics.GetPlayerPawn` 0)) 0.0 500.0))

(fn `Stop Audio`
  (`AudioComponent.FadeOut` (`self.HissingGasAudio`) 2.5 0.0 "Linear")
  (`AudioComponent.Stop` (`self.CoughingAudio`)))

(fn `UserConstructionScript`)