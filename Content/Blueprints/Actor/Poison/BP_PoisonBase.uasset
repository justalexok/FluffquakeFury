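; BP_PoisonBase is a poison fog actor that reacts when poison is released in the game.
; On BeginPlay it caches the FogArea's world scale and binds to the FQF game mode's OnPoisonReleased event.
; When that fires, it applies a green fog material, plays a gas hiss and slows global time, with no reset here.
; A timeline then drives ScaleFogArea, scaling the fog relative to its cached size.
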(event `self.ReceiveBeginPlay`
  (`|ExecutionSequence`
    (:`then_0`
      (set `self.TargetScale` (`SceneComponent.K2_GetComponentScale` (`self.FogArea`))))
    (:`then_1`
      (bind _returnvalue (`FQFBlueprintFunctionLibrary.GetFQFGameMode` (`GameplayStatics.GetPlayerPawn` 0)))
      (bind _asbp_fqfgame_mode_base (cast `/Game/Blueprints/Game/BP_FQFGameModeBase` _returnvalue))
      (bind _output_get (set `self.BP FQFGame Mode Base` _asbp_fqfgame_mode_base))
      (add `/Game/Blueprints/Game/BP_FQFGameModeBase.OnPoisonReleased` _output_get (delegate `OnPoisonReleased_Event`)))))

(event `OnPoisonReleased_Event`
  ;[0.04224 1 0.1665] On Poison Released
  (`PrimitiveComponent.SetMaterial` (`self.FogArea`) 0 "/Game/Blueprints/Actor/Poison/M_GreenFog.M_GreenFog")
  (`GameplayStatics.PlaySoundAtLocation` "/Game/AGContent/SFX/Attacks/Poison/HissingGas_Meta.HissingGas_Meta" (`self.K2_GetActorLocation`) (struct) 1.0 1.0 0.0 null null null null)
  (`GameplayStatics.SetGlobalTimeDilation` 0.3)
  (bind (_direction _scale) (`Timeline|Timeline`)
    (:`Update`
      (`self.ScaleFogArea` _scale _scale _scale))))

(fn `ScaleFogArea`
  (params (X :type "Float (double-precision)") (Y :type "Float (double-precision)") (Z :type "Float (double-precision)"))
  (bind (_targetscale_x _targetscale_y _targetscale_z) (`KismetMathLibrary.BreakVector` (`self.TargetScale`)))
  (bind _targetscale_x_2 (`KismetMathLibrary.BreakVector` (`self.TargetScale`)))
  (bind (_targetscale_x_3 _targetscale_y_2) (`KismetMathLibrary.BreakVector` (`self.TargetScale`)))
  (`SceneComponent.SetWorldScale3D` (`self.FogArea`) (`KismetMathLibrary.MakeVector` (* Z _targetscale_x_2) (* X _targetscale_y_2) (* _targetscale_z Y))))

(fn `UserConstructionScript`)