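; BP_ProjectilePillow is a pillow projectile that spins around its yaw axis every tick and triggers a poison impact.
; On the first sphere overlap with an actor other than itself or the player pawn, it spawns the poison Niagara effect and plays an explosion sound.
; It sends the DamageType.Poison gameplay event to the player pawn, not the overlapped actor, then destroys itself after a short delay.
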(event `self.ReceiveActorBeginOverlap`
  (params (OtherActor :type "Actor Object Reference")))

(event `self.ReceiveTick`
  (params (DeltaSeconds :type "Float (single-precision)"))
  (`self.K2_SetActorRotation` (`KismetMathLibrary.ComposeRotators` (`self.K2_GetActorRotation`) (`KismetMathLibrary.MakeRotator` 0.0 0.0 (* DeltaSeconds 500.0)))))

(event `self.Sphere.OnComponentBeginOverlap`
  (params (OverlappedComponent :type "PrimitiveComponent Object Reference") (OtherActor :type "Actor Object Reference") (OtherComp :type "PrimitiveComponent Object Reference") (OtherBodyIndex :type Integer) (bFromSweep :type Boolean) (SweepResult :type "HitResult Structure (by ref)"))
  (if (and (!= OtherActor self) (!= OtherActor (`GameplayStatics.GetPlayerPawn` 0)))
    (`/Engine/EditorBlueprintResources/StandardMacros.DoOnce` false
      (:`Completed`
        (`NiagaraFunctionLibrary.SpawnSystemAtLocation` "/Game/AGContent/Niagara/NS_PoisonPillowImpact.NS_PoisonPillowImpact" (`self.K2_GetActorLocation`))
        (`GameplayStatics.PlaySound2D` "/Game/AGContent/SFX/Attacks/Poison/smallExplosion.smallExplosion" 1.0 1.0 0.0 null null)
        (`AbilitySystemBlueprintLibrary.SendGameplayEventToActor` (`GameplayStatics.GetPlayerPawn` 0) (struct :`TagName` "DamageType.Poison"))
        (`KismetSystemLibrary.Delay` 2.0)
        (`self.K2_DestroyActor`)))))

(fn `UserConstructionScript`)