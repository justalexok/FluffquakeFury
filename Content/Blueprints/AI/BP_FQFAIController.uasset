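; AI controller with an AI Perception component and a helper for checking whether it senses a given actor.
; CanSenseActor scans the actor's last sensed stimuli for one matching the chosen sense, with sight mapped, and returns its success flag and stimulus.
; The perception update event is empty.
; Disconnected logic would write player visibility to the pawn's CanISeePlayer blackboard key and handle sight detection, but it never runs.
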(event `self.AIPerception.OnPerceptionUpdated`
  (params (UpdatedActors :type "Array of Actor Object Reference (by ref)")))

(fn `CanSenseActor`
  (params (Actor :type "Actor Object Reference") (Sense :type "/Game/Blueprints/AI/E_AISense Enum" :default "NewEnumerator0"))
  (returns (SensedPlayer :type Boolean) (Stimulus :type "AIStimulus Structure"))
  (bind _info (`AIPerceptionComponent.GetActorsPerception` (`self.AIPerception`) Actor))
  (for _array_element (`.LastSensedStimuli` (break `ActorPerceptionBlueprintInfo` _info))
    (bind _returnvalue (`AIPerceptionSystem.GetSenseClassForStimulus` _array_element))
    (if (== _returnvalue (select `/Game/Blueprints/AI/E_AISense` Sense :`NewEnumerator1` "/Script/AIModule.AISense_Sight" :!type "Object Class Reference"))
      (return (`.bSuccessfullySensed` (break `AIStimulus` _array_element)) _array_element))))

(fn `UserConstructionScript`)