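; BP_ChainedMeshSet is a construction-script actor that procedurally builds a chain of static meshes with random decorations.
; From a start mesh, it adds random meshes, each parented to the previous at an attach offset so yaw accumulates from random, constant and index-scaled terms.
; Each link gets a random decoration using that entry's transform.
; GetRandomOffsetVector is meant to jitter decoration positions, but its random vector is left unconnected.
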(fn `UserConstructionScript`
  (locals (LastComponentRef :type "SceneComponent Object Reference") (RandomDecoration :type "/Game/Kids_Toys/Blueprints/S_ChainedMeshDecoration Structure"))
  (bind _lastcomponentref (`local.LastComponentRef`))
  (bind _staticmesh (`self.StaticMesh`))
  (bind _chainedmesh (`self.ChainedMesh`))
  ;[1 1 1] Init
  (`StaticMeshComponent.SetStaticMesh` _staticmesh (`self.StartMesh`))
  (set `local.LastComponentRef` _staticmesh)
  (for _index (range (`self.ChainLength`))
    ;[1 1 1] Add new chain element
    (bind _returnvalue (`AddComponent|NODE_AddStaticMeshComponent-1` :`bManualAttachment` true :`RelativeTransform` (`KismetMathLibrary.MakeTransform` (+ (`KismetMathLibrary.InverseTransformLocation` (`SceneComponent.K2_GetComponentToWorld` _lastcomponentref) (`SceneComponent.K2_GetComponentLocation` _lastcomponentref)) (`KismetMathLibrary.SelectVector` (`self.StartMeshAttachOffset`) (`self.ChainedMeshAttachOffset`) (== _index 0))) (`KismetMathLibrary.MakeRotator` 0.0 0.0 (+ (+ (`KismetMathLibrary.RandomFloatInRange` (`self.RandomRotationMin`) (`self.RandomRotationMax`)) (`self.ConstantRotation`)) (* _index (`self.IndexMultipliedRotation`)))))))
    (`SceneComponent.K2_AttachToComponent` _returnvalue (`local.LastComponentRef`) "None" "KeepRelative" "KeepRelative" "KeepRelative" true)
    (set `local.LastComponentRef` _returnvalue)
    (`StaticMeshComponent.SetStaticMesh` _returnvalue (`|GetArrayItem` _chainedmesh (`.Index` (`/Game/Kids_Toys/Blueprints/BP_GetRandomFromArray.GetRandomFromArray` _chainedmesh))))
    ;[1 1 1] Attach random decoration
    (bind _output_get (set `local.RandomDecoration` (`/Game/Kids_Toys/Blueprints/BP_GetRandomFromArray.GetRandomFromArray` (`self.Decorations`))))
    (bind _returnvalue_2 (`AddComponent|NODE_AddStaticMeshComponent-2` :`bManualAttachment` true :`RelativeTransform` (`KismetMathLibrary.MakeTransform` (+ (.location (`.Transform_12_42D5F41D4093178706400BBACEA42797` (break `/Game/Kids_Toys/Blueprints/S_ChainedMeshDecoration` _output_get))) (`KismetMathLibrary.MakeVector` (`KismetMathLibrary.RandomFloatInRange` (.x (`.RandomOffsetMin_20_0DD2F28349EE1BFB61D37A9C612B16CA` (break `/Game/Kids_Toys/Blueprints/S_ChainedMeshDecoration` _output_get))) (.x (`.RandomOffsetMax_22_118A23754E9D3785F9BB70B48965C9DF` (break `/Game/Kids_Toys/Blueprints/S_ChainedMeshDecoration` _output_get)))) (`KismetMathLibrary.RandomFloatInRange` (.y (`.RandomOffsetMin_20_0DD2F28349EE1BFB61D37A9C612B16CA` (break `/Game/Kids_Toys/Blueprints/S_ChainedMeshDecoration` _output_get))) (.y (`.RandomOffsetMax_22_118A23754E9D3785F9BB70B48965C9DF` (break `/Game/Kids_Toys/Blueprints/S_ChainedMeshDecoration` _output_get)))) (`KismetMathLibrary.RandomFloatInRange` (.z (`.RandomOffsetMin_20_0DD2F28349EE1BFB61D37A9C612B16CA` (break `/Game/Kids_Toys/Blueprints/S_ChainedMeshDecoration` _output_get))) (.z (`.RandomOffsetMax_22_118A23754E9D3785F9BB70B48965C9DF` (break `/Game/Kids_Toys/Blueprints/S_ChainedMeshDecoration` _output_get)))))) (.rotation (`.Transform_12_42D5F41D4093178706400BBACEA42797` (break `/Game/Kids_Toys/Blueprints/S_ChainedMeshDecoration` _output_get))) (.scale (`.Transform_12_42D5F41D4093178706400BBACEA42797` (break `/Game/Kids_Toys/Blueprints/S_ChainedMeshDecoration` _output_get))))))
    (`SceneComponent.K2_AttachToComponent` _returnvalue_2 (`local.LastComponentRef`) "None" "KeepRelative" "KeepRelative" "KeepRelative" true)
    (`StaticMeshComponent.SetStaticMesh` _returnvalue_2 (break `/Game/Kids_Toys/Blueprints/S_ChainedMeshDecoration` _output_get))))