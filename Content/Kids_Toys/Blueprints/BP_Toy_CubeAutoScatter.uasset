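; Toy cube prop that procedurally scatters static mesh cubes within a configurable area in its construction script.
; Each cube gets a random XY point at fixed height, with roll and pitch drawn from a rotation pool and random yaw.
; A CubeOverlap test against WorldStatic objects rejects occupied spots, retrying a few times before skipping that cube.
; Placed cubes are set to WorldStatic, so later placements avoid them.
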(fn `GetRandomFromArray`
  (params (Array :type "Array of Integer"))
  (returns (Output :type Integer))
  (return (`|GetArrayItem` Array (`KismetMathLibrary.RandomIntegerInRange` 0 (- (`KismetArrayLibrary.Array_Length` Array) 1)))))

(fn `GetRandomPoint`
  (returns (ReturnValue :type "Vector Structure"))
  (bind (_scatter_volume_size_x _scatter_volume_size_y) (`KismetMathLibrary.BreakVector2D` (`self.Scatter Volume Size`)))
  (bind (_returnvalue_x _returnvalue_y) (`KismetMathLibrary.BreakVector` (`KismetMathLibrary.RandomPointInBoundingBox` (0.0 0.0 0.0) (`KismetMathLibrary.MakeVector` _scatter_volume_size_x _scatter_volume_size_y))))
  (return (`KismetMathLibrary.MakeVector` _returnvalue_x _returnvalue_y 3.0)))

(fn `GetRandomRotator`
  (returns (ReturnValue :type "Rotator Structure"))
  (bind (_returnvalue_roll _returnvalue_pitch _returnvalue_yaw) (`KismetMathLibrary.BreakRotator` (`KismetMathLibrary.RandomRotator` false)))
  (bind _rotationpool (`self.RotationPool`))
  (bind _output (`self.GetRandomFromArray` _rotationpool))
  (bind _output_2 (`self.GetRandomFromArray` _rotationpool))
  (return (`KismetMathLibrary.MakeRotator` (`KismetMathLibrary.Conv_IntToDouble` _output) (`KismetMathLibrary.Conv_IntToDouble` _output_2) _returnvalue_yaw)))

(fn `UserConstructionScript`
  (locals (BPCubeASActorClass :type "Actor Class Reference") (NewLocalVar_0 :type "Vector Structure" :default (0.0 0.0 0.0)))
  (for _ (range 1 (`self.Number of scattered objects`))
    (set `self.PlacementRetryCount` 0)
    (bind _returnvalue (`self.GetRandomRotator` :!label _label))
    (bind _returnvalue_2 (`self.GetRandomPoint`))
    (bind (_outcomponents _returnvalue_3) (`KismetSystemLibrary.ComponentOverlapComponents` (`self.CubeOverlap`) (`KismetMathLibrary.MakeTransform` (`KismetMathLibrary.TransformLocation` (`SceneComponent.K2_GetComponentToWorld` (`self.DefaultSceneRoot`)) _returnvalue_2) _returnvalue) (`|MakeArray` "ObjectTypeQuery1" :!type "EObjectTypeQuery Enum")))
    (if _returnvalue_3
      (bind _result (`/Engine/EditorBlueprintResources/StandardMacros.IncrementInt` (`self.PlacementRetryCount`))
        (:`  `
          (if (<= _result 5)
            (goto _label))))
      (else
        (bind _returnvalue_4 (`AddComponent|NODE_AddStaticMeshComponent-3` :`RelativeTransform` (`KismetMathLibrary.MakeTransform` _returnvalue_2 _returnvalue)))
        (`PrimitiveComponent.SetCollisionObjectType` _returnvalue_4 "ECC_WorldStatic")))))