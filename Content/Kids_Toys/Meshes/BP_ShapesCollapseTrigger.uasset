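; Trigger actor that collapses the toy shapes when a BP_Ball enters its collision component.
; On overlap it enables physics on every BP_ToyShape in the level and calls StruckByBall on each.
; It then spawns a BP_ky_healAura effect at GroundPoint, repeating every second through a Delay loop with no exit condition.
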(event `self.CollisionComponent.OnComponentBeginOverlap`
  (params (OverlappedComponent :type "PrimitiveComponent Object Reference") (OtherActor :type "Actor Object Reference") (OtherComp :type "PrimitiveComponent Object Reference") (OtherBodyIndex :type Integer) (bFromSweep :type Boolean) (SweepResult :type "HitResult Structure (by ref)"))
  (cast `/Game/Kids_Toys/Meshes/BP_Ball` OtherActor)
  (bind _outactors (`GameplayStatics.GetAllActorsOfClass` "/Game/Kids_Toys/Meshes/BP_ToyShape.BP_ToyShape_C"))
  (for _array_element _outactors
    (`PrimitiveComponent.SetSimulatePhysics` (`StaticMeshActor.StaticMeshComponent` _array_element) true)
    (`/Game/Kids_Toys/Meshes/BP_ToyShape.Struck by Ball` _array_element))
  (`|SpawnActorFromClass` "/Game/AGContent/Niagara/FXVarietyPack/Blueprints/BP_ky_healAura.BP_ky_healAura_C" (`KismetMathLibrary.Conv_VectorToTransform` (`SceneComponent.K2_GetComponentLocation` (`self.GroundPoint`))) "Undefined" "MultiplyWithRoot" null null :!label _label)
  (`KismetSystemLibrary.Delay` 1.0)
  (goto _label))

(fn `UserConstructionScript`)