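; BP_ToyShape is a toy shape actor that reacts to being struck by a ball.
; Its construction script gives the static mesh a yaw picked at random from the Rotations array.
; The StruckbyBall event plays a falling-blocks sound at the mesh, limited by concurrency settings, then destroys the actor after a short random delay.
; Nothing in this Blueprint calls that event, and BeginPlay, overlap and Tick are unused.
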(event `Struck by Ball`
  (`GameplayStatics.PlaySoundAtLocation` "/Game/AGContent/SFX/BlocksFalling.BlocksFalling" (`SceneComponent.K2_GetComponentLocation` (`self.StaticMeshComponent`)) (struct) 2.0 1.0 0.0 null "/Game/AGContent/SFX/NewSoundConcurrency.NewSoundConcurrency" self null)
  (`KismetSystemLibrary.Delay` (`KismetMathLibrary.RandomFloatInRange` 1.0 3.0))
  (`self.K2_DestroyActor`))

(fn `UserConstructionScript`
  (locals (Rotations :type "Array of Integer"))
  (`SceneComponent.K2_SetRelativeRotation` (`self.StaticMeshComponent`) (`KismetMathLibrary.MakeRotator` 0.0 0.0 (`KismetMathLibrary.Conv_IntToDouble` (`KismetArrayLibrary.Array_Random` (`local.Rotations`)))) false false))